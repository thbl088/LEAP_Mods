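; Squid variant of the ProjectX character that punishes movement while moving is not allowed.
; Each Tick runs the parent logic, then checks AllowedToMove and whether the CharacterMovement velocity is near zero.
; If it moves while disallowed, it applies heavy damage to itself using the airstrike bomb damage type.
; The construction script only calls the parent.
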(event `self.ReceiveTick`
  (params (DeltaSeconds :type "Float (single-precision)"))
  (`parent.ReceiveTick` DeltaSeconds)
  (if (`self.AllowedToMove`)
    _
    (elif (not (== (`MovementComponent.Velocity` (`self.CharacterMovement`)) (0.0 0.0 0.0)))
      (`GameplayStatics.ApplyDamage` self 1000.0 null null "/Game/Blueprints/Gameplay/DamageTypes/DT_Airstrike_Bomb.DT_Airstrike_Bomb_C"))))

(fn `UserConstructionScript`
  (`parent.UserConstructionScript`))