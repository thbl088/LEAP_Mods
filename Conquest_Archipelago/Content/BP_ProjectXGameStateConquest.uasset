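; Conquest game state Blueprint that drives match music and broadcast warnings from team ticket counts and remaining time.
; Music moves from a match-start cue and playlist to a one-shot tension cue near the end, then victory or defeat, gated to cosmetic-capable instances.
; Ticket updates broadcast one-time low-ticket and halfway warnings, each using a single flag shared by both teams.
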(event `self.ReceiveBeginPlay`
  (bind _returnvalue (`GameplayStatics.GetPlayerController` 0))
  (`|ExecutionSequence`
    (:`then_0`
      (`KismetSystemLibrary.K2_SetTimerDelegate` (`|CreateDelegate` :!event `CheckMatchEndingSoon`) 2.0 true)
      (add `self.OnWinningTeamSetEvent` (`|CreateDelegate` :!event `OnWinnerDecided`)))
    (:`then_1`
      (`/Engine/EditorBlueprintResources/StandardMacros.IsValid` _returnvalue
        (:`Is Valid`
          (if (`Controller.IsLocalPlayerController` _returnvalue)
            (add `self.OnTeamTicketsChanged` (delegate `OnTicketCountChanged`))))))))

(event `OnTicketCountChanged` :!signature `self.OnTeamTicketsChanged`
  (params (Tickets :type "Array of TeamTicketInfo Structure (by ref)"))
  ;[1 1 1] Play music that increases in intensity as a match winds down, either due to score or timer
  (`self.OnTicketCountUpdate_1`)
  (if (or (<= (`self.GetTicketCount` 0) 38) (<= (`self.GetTicketCount` 1) 38))
    (`/Engine/EditorBlueprintResources/StandardMacros.DoOnce` false :!label _label
      (:`Completed`
        (`/Engine/EditorBlueprintResources/StandardMacros.Can Execute Cosmetic Events`
          (:`True`
            (`MusicPlayer.Play` (`MusicPlayer.GetMusicPlayer`) (make `TrackPlayInfo` "/Game/Audio/Music/Stingers/TensionBuilder_Cue.TensionBuilder_Cue" 3.0 3.0 1.0 false (0.0 0.0) false))))))))

(event `CheckMatchEndingSoon`
  ;[1 1 1] Play music that increases in intensity as a match winds down, either due to score or timer
  (if (<= (`KismetMathLibrary.FTrunc` (`self.GetMatchTimeRemaining`)) 148)
    (goto _label)))

(event `self.OnPlayerPawnSpawned`
  (params (Character :type "ProjectXCharacter Object Reference"))
  (bind _returnvalue (`MusicPlayer.GetMusicPlayer`))
  (`/Engine/EditorBlueprintResources/StandardMacros.Can Execute Cosmetic Events`
    (:`True`
      (`/Engine/EditorBlueprintResources/StandardMacros.DoOnce` false
        (:`Completed`
          (`KismetSystemLibrary.Delay` 1.0)
          (`MusicPlayer.Play` _returnvalue (make `TrackPlayInfo` "/Game/Audio/Music/Stingers/MatchStart_Cue.MatchStart_Cue" 0.0 1.0 1.0 true (50.0 150.0) false))
          (`MusicPlayer.SetTrackList` _returnvalue (`self.MusicPlaylist`) true false false))))))

(event `OnTicketCountUpdate_1`
  (`self.SendLowTicketWarning`)
  (`self.CheckMatchHalfwayMark`))

(event `SendLowTicketWarning`
  (`|ExecutionSequence`
    (:`then_0`
      (if (and (not (`self.bSentLowTicketWarning`)) (> (`KismetMathLibrary.FFloor` (* (`self.GetStartingTicketCount` 0) 0.25)) (`self.GetTicketCount` 0)))
        (set `self.bSentLowTicketWarning` true)
        (`BroadcastMessage.BroadcastServerMessage` "/Game/Blueprints/BroadcastMessage/Gamemodes/BaseControl/BP_BroadcastMessage_BC_TeamLowTicketCount.BP_BroadcastMessage_BC_TeamLowTicketCount_C" 1)))
    (:`then_1`
      (if (and (> (`KismetMathLibrary.FFloor` (* (`self.GetStartingTicketCount` 1) 0.25)) (`self.GetTicketCount` 1)) (not (`self.bSentLowTicketWarning`)))
        (set `self.bSentLowTicketWarning` true)
        (`BroadcastMessage.BroadcastServerMessage` "/Game/Blueprints/BroadcastMessage/Gamemodes/BaseControl/BP_BroadcastMessage_BC_TeamLowTicketCount.BP_BroadcastMessage_BC_TeamLowTicketCount_C")))))

(event `OnWinnerDecided` :!signature `self.OnWinningTeamSetEvent`
  (params (Winner :type Integer))
  (`/Engine/EditorBlueprintResources/StandardMacros.Can Execute Cosmetic Events`
    (:`True`
      (if (== (`self.MatchState`) "WaitingPostMatch")
        (if (!= Winner -1)
          (`MusicPlayer.Play` (`MusicPlayer.GetMusicPlayer`) (make `TrackPlayInfo` (select `bool` (== Winner (`self.GetTeamStatic` (`GameplayStatics.GetPlayerPawn` 0))) :`false` "/Game/Audio/Music/Stingers/GameOver_Defeat_Cue.GameOver_Defeat_Cue" :`true` "/Game/Audio/Music/Stingers/GameOver_Victory_Cue.GameOver_Victory_Cue" :!type "SoundBase Object Reference") 3.0 3.0 1.0 false (0.0 0.0) false))
          (else
            (`MusicPlayer.Stop` (`MusicPlayer.GetMusicPlayer`) 1.0)))))))

(event `CheckMatchHalfwayMark`
  (bind _returnvalue (<= (`KismetMathLibrary.FTrunc` (`self.GetMatchTimeRemaining`)) (`KismetMathLibrary.FTrunc` (* (`self.GetMatchLengthStatic`) 0.5))))
  (`|ExecutionSequence`
    (:`then_0`
      (if (or (<= (`self.GetTicketCount` 0) (`KismetMathLibrary.FFloor` (* (`self.GetStartingTicketCount` 0) 0.5))) _returnvalue)
        (if (not (`self.bSentGameEndingSoonWarning`))
          (set `self.bSentGameEndingSoonWarning` true)
          (`BroadcastMessage.BroadcastServerMessage` "/Game/Blueprints/BroadcastMessage/Gamemodes/BaseControl/BP_BroadcastMessage_BC_MatchHalfWayWarning.BP_BroadcastMessage_BC_MatchHalfWayWarning_C" 1))))
    (:`then_1`
      (if (or (<= (`self.GetTicketCount` 1) (`KismetMathLibrary.FFloor` (* (`self.GetStartingTicketCount` 1) 0.5))) _returnvalue)
        (if (not (`self.bSentGameEndingSoonWarning`))
          (set `self.bSentGameEndingSoonWarning` true)
          (`BroadcastMessage.BroadcastServerMessage` "/Game/Blueprints/BroadcastMessage/Gamemodes/BaseControl/BP_BroadcastMessage_BC_MatchHalfWayWarning.BP_BroadcastMessage_BC_MatchHalfWayWarning_C"))))))

(fn `UserConstructionScript`)