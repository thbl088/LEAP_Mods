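; Player character Blueprint with a Smash Bros-style damage percentage that makes hits knock the character farther as it accumulates.
; AddPourcentage records the last hit's damage and adds it to BumpPourcentage.
; CalculateKnockback combines both with Weight in a Smash-like formula, which Bump applies along a direction as a velocity-change impulse using neutral attack parameters.
; GetBumpForce separately samples BumpCurve by percentage and is not used by Bump.
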(fn `AddPourcentage`
  (params (Damage :type "Float (double-precision)"))
  (bind _output_get (set `self.PreviousAttackPourcentage` Damage))
  (set `self.BumpPourcentage` (+ _output_get (`self.BumpPourcentage`))))

(fn `Bump`
  (params (Direction :type "Vector Structure"))
  (bind _knockbacck (`self.CalculateKnockback` 1.0 1.0))
  (`CharacterMovementComponent.AddImpulse` (`self.CharacterMovement`) (* Direction _knockbacck) true))

(fn `CalculateKnockback`
  (params (`attack base knockback` :type "Float (double-precision)") (`Attack knockback scaling` :type "Float (double-precision)") (`Other ratios` :type "Float (double-precision)" :default 1.0))
  (returns (Knockbacck :type "Float (double-precision)"))
  (return (* (+ (* (+ (* (* (+ (/ (`self.BumpPourcentage`) 10.0) (/ (* (`self.BumpPourcentage`) (`self.PreviousAttackPourcentage`)) 20.0)) (/ 200.0 (+ (`self.Weight`) 100.0))) 1.4) 18.0) `Attack knockback scaling`) `attack base knockback`) `Other ratios`)))

(fn `GetBumpForce`
  (returns (BumpForce :type "Float (double-precision)"))
  (return (`CurveFloat.GetFloatValue` (`self.BumpCurve`) (`self.BumpPourcentage`))))

(fn `UserConstructionScript`
  (`parent.UserConstructionScript`))