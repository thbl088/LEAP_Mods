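; Client-side rocket-bump projectile that knocks characters away from its point of impact.
; On hit, it gathers targets within a bump radius around its own location.
; Each target that casts to the ProjectX character has Bump called with a normalized direction pointing from the projectile to that character, producing a radial push.
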(event `self.ReceiveHit`
  (params (MyComp :type "PrimitiveComponent Object Reference") (Other :type "Actor Object Reference") (OtherComp :type "PrimitiveComponent Object Reference") (bSelfMoved :type Boolean) (HitLocation :type "Vector Structure") (HitNormal :type "Vector Structure") (NormalImpulse :type "Vector Structure") (Hit :type "HitResult Structure (by ref)"))
  (`self.BumpArea`))

(fn `BumpArea`
  (locals (BumpedPlayer :type "/SuperSmashMerc/Blueprints/PlayerClasses/BP_ProjectXCharacter_SSM Object Reference"))
  (for _array_element (`ProjectXGameplayStatics.GetTargetsInRadius` (`self.K2_GetActorLocation` self) (`self.RadiusBump`))
    (bind _asbp_project_xcharacter_ssm (cast `/SuperSmashMerc/Blueprints/PlayerClasses/BP_ProjectXCharacter_SSM` _array_element))
    (set `local.BumpedPlayer` _asbp_project_xcharacter_ssm)
    (`/SuperSmashMerc/Blueprints/PlayerClasses/BP_ProjectXCharacter_SSM.Bump` (`local.BumpedPlayer`) (`KismetMathLibrary.Normal` (- (`self.K2_GetActorLocation` (`local.BumpedPlayer`)) (`self.K2_GetActorLocation` self))))))

(fn `UserConstructionScript`)