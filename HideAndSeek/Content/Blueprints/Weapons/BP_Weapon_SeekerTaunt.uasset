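; Seeker taunt weapon that plays a random sound on the owning character and gives it a temporary movement speed boost when fired.
; Fire runs the parent logic, then destroys the previous taunt audio and attaches a new attenuated sound to the character's mesh.
; It caches the max walk speed, multiplies it by SpeedBoost, and restores the cached value after a delay of DurationSpeedBoost.
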(event `self.K2_Fire`
  (params (Mode :type Byte))
  (`parent.K2_Fire` Mode)
  (bind _asbp_project_xcharacter (cast `/Game/Blueprints/Gameplay/PlayerClasses/BP_ProjectXCharacter` (`self.GetOwner`)))
  (`self.K2_DestroyComponent` (`self.SoundCue`))
  (bind _returnvalue (`GameplayStatics.SpawnSoundAttached` (`KismetArrayLibrary.Array_Random` (`self.Sound`)) (`Character.Mesh` _asbp_project_xcharacter) "None" (0.0 0.0 0.0) (struct) "KeepRelativeOffset" true 1.5 1.0 0.0 "/Game/Audio/Attenuations/Explosion_Medium_Attenuation.Explosion_Medium_Attenuation" null))
  (set `self.SoundCue` _returnvalue)
  (bind _charactermovement (`Character.CharacterMovement` _asbp_project_xcharacter))
  (bind _maxwalkspeed (`CharacterMovementComponent.MaxWalkSpeed` _charactermovement))
  (set `self.Max Walk Speed` _maxwalkspeed)
  (set `CharacterMovementComponent.MaxWalkSpeed` (* _maxwalkspeed (`self.speedBoost`)) _charactermovement)
  (`KismetSystemLibrary.Delay` (`self.durationSpeedBoost`))
  (set `CharacterMovementComponent.MaxWalkSpeed` (`self.Max Walk Speed`) _charactermovement))