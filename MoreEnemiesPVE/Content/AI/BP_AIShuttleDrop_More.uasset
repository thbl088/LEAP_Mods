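; AI shuttle drop pod variant that removes its interactable and spawns AI from spawners on its podium, then destroys itself on the server after ten seconds.
; On initialization, the server starts each spawner in a staggered delayed loop, using child-actor spawners unless runtime ones exist.
; K2_BeginSpawning builds runtime spawners from an override character list, cloning the template spawner's class and attaching them at preset offsets.
; StopSpawning halts spawners, deactivates and destroys the pod.
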(event `self.ReceiveBeginPlay`
  (`parent.ReceiveBeginPlay`)
  (`|ExecutionSequence`
    (:`then_0`
      (bind _interactable (`self.Interactable`)
        (:`then`
          (`ActorComponent.K2_DestroyComponent` _interactable))
        (:`else`)))
    (:`then_1`
      (`/Engine/EditorBlueprintResources/ActorMacros.Switch Has Authority`
        (:`Authority`
          (`KismetSystemLibrary.Delay` 10.0)
          (`self.K2_DestroyActor`))))))

(event `self.OnInitialized`
  (`parent.OnInitialized`)
  (`/Engine/EditorBlueprintResources/ActorMacros.Switch Has Authority`
    (:`Authority`
      (if (not (`self.bDeactivated`))
        (bind _returnvalue (`self.GetSpawnChildren`))
        (bind _array_element (`/Game/Blueprints/Functions/ProjectXMacros.ForEachLoopDelayed` _returnvalue :!label _label)
          (:`Loop Body`
            (`self.BeginSpawning` _array_element)
            (`self.SpawnNext`)))))))

(event `SpawnNext`
  (`KismetSystemLibrary.Delay` 0.1)
  (goto _label :!via `Next Body`))

(event `self.StopSpawning`
  (bind _array_element (`/Game/Blueprints/Functions/ProjectXMacros.ForEachLoopDelayed` (`self.RuntimeSpawns`))
    (:`Loop Body`
      (`self.StopSpawning` _array_element)
      (set `self.bDeactivated` true)
      (`self.K2_DestroyActor`))))

(fn `GetSpawnChildren`
  (returns (ReturnValue :type "Array of SpawnInterface Interface"))
  (if (not (> (`KismetArrayLibrary.Array_Length` (`self.RuntimeSpawns`)) 0))
    (for _array_element (`SceneComponent.GetChildrenComponents` (`self.SM_EpicLoorDrop_Podium`) false)
      (bind _aschild_actor_component (cast `ChildActorComponent` _array_element))
      (bind _asspawn_interface (cast `SpawnInterface` (`ChildActorComponent.ChildActor` _aschild_actor_component)))
      (`KismetArrayLibrary.Array_Add` (`self.RuntimeSpawns`) _asspawn_interface)))
  (return (`self.RuntimeSpawns`)))

(fn `K2_BeginSpawning`
  (params (SpawnOverrideList :type "Array of Actor Class Reference (by ref)"))
  (`KismetArrayLibrary.Array_Clear` (`self.RuntimeSpawns`))
  (for (_array_element _array_index) SpawnOverrideList
    (bind _asproject_xcharacter (castclass `ProjectXCharacter` _array_element))
    (bind _returnvalue (`|SpawnActorFromClass` (`GameplayStatics.GetObjectClass` (cast `ProjectXAISpawner` (`ChildActorComponent.ChildActor` (`self.AISpawnerA_P1`)) :!pure true)) (`SceneComponent.K2_GetComponentToWorld` (`self.AISpawnerA_P1`)) "Undefined" "OverrideRootScale" null null))
    (set `ProjectXAISpawner.AIToSpawn` _asproject_xcharacter _returnvalue)
    (set `ProjectXAISpawner.SpawnDelay` 0.0 _returnvalue)
    (set `ProjectXAISpawner.bExecuteImmediately` false _returnvalue)
    (set `ProjectXAISpawner.bExecuteOnMatchStart` false _returnvalue)
    (`self.K2_AttachToComponent` _returnvalue (`self.SM_EpicLoorDrop_Podium`) "None" "SnapToTarget" "SnapToTarget" "SnapToTarget" false)
    (if (`KismetArrayLibrary.Array_IsValidIndex` (`self.SpawnRelativeLocations`) _array_index)
      (`self.K2_SetActorRelativeLocation` _returnvalue (`|GetArrayItem` (`self.SpawnRelativeLocations`) _array_index) false false)
      (`KismetArrayLibrary.Array_Add` (`self.RuntimeSpawns`) _returnvalue)))
  (`ActorComponent.K2_DestroyComponent` (`self.AISpawnerA_P1`))
  (return))

(fn `UserConstructionScript`
  (`parent.UserConstructionScript`))