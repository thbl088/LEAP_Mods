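; Nerfed repair gun affliction that supplies healing feedback on the affected character; it applies no healing itself.
; Start shows a healing overlay for the local player or an attached aura particle for others, and enables ticking after one interval.
; Tick plays a sound and refreshes these below max health, removing the aura at full; End clears both.
; TakeDamage computes a damage-tiered heal delay that goes unused, returning damage unchanged.
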(event `self.K2_Start`
  (bind _returnvalue (`self.GetOwningCharacter`))
  (`|ExecutionSequence`
    (:`then_0`
      (`KismetSystemLibrary.Delay` (`self.GetComponentTickInterval`))
      (`self.SetComponentTickEnabled` true))
    (:`then_1`
      (`self.HealParticle` :!label _label
        (:`then`)
        (:`else`
          (`/Engine/EditorBlueprintResources/StandardMacros.IsValid` _returnvalue
            (:`Is Valid`
              (if (`Pawn.IsLocallyControlled` _returnvalue)
                (`self.Widget`
                  (:`then`)
                  (:`else`
                    (bind _returnvalue_2 (`|CreateWidget` "/Game/Blueprints/UI/W_HealingOverlay.W_HealingOverlay_C" (`GameplayStatics.GetPlayerController` 0)))
                    (bind _output_get (set `self.Widget` _returnvalue_2))
                    (`UserWidget.AddToViewport` _output_get 0)))
                (elif (not (`KismetSystemLibrary.IsDedicatedServer`))
                  (bind _returnvalue_3 (`GameplayStatics.SpawnEmitterAttached` "/Game/ThirdPartyAssets/FXVarietyPack/Particles/P_HealAura.P_HealAura" (`Character.Mesh` _returnvalue) "SpineSocket" (0.0 0.0 0.0) (struct :`Pitch` -90.0) (1.0 1.0 1.0) "SnapToTarget" false "AutoRelease"))
                  (set `self.HealParticle` _returnvalue_3))))))))))

(event `self.ReceiveTick`
  (params (DeltaSeconds :type "Float (single-precision)"))
  (bind _returnvalue (`self.GetOwningCharacter`))
  (`/Engine/EditorBlueprintResources/StandardMacros.IsValid` _returnvalue
    (:`Is Valid`
      (if (< (`HealthInterface.GetHealth` _returnvalue) (`HealthInterface.GetMaxHealth` _returnvalue))
        (`GameplayStatics.SpawnSoundAttached` "/Game/Audio/Weapons/RepairGun/Healing_Beam_Positive_Hit.Healing_Beam_Positive_Hit" (`Character.Mesh` _returnvalue) "None" (0.0 0.0 0.0) (struct) "KeepRelativeOffset" false 1.0 1.0 0.0 null null)
        (goto _label)
        (else
          (bind _healparticle (`self.HealParticle` :!label _label_2)
            (:`then`
              (`self.Deactivate` _healparticle)
              (`self.K2_DestroyComponent` _healparticle)
              (set `self.HealParticle` null))
            (:`else`)))))))

(event `self.K2_End`
  (bind _widget (`self.Widget`)
    (:`then`
      (`Widget.RemoveFromParent` _widget)
      (goto _label_2))
    (:`else`
      (goto _label_2))))

(fn `SetHealDelay`
  (params (Damage :type "Float (double-precision)"))
  (locals (NewHealDelay :type "Float (double-precision)"))
  (if (< Damage 5.0)
    (set `local.NewHealDelay` 0.1)
    (elif (< Damage 10.0)
      (set `local.NewHealDelay` 0.2)
      (elif (< Damage 20.0)
        (set `local.NewHealDelay` 0.4)
        (elif (< Damage 40.0)
          (set `local.NewHealDelay` 0.8)
          (else
            (set `local.NewHealDelay` 1.0))))))
  (if (> (`local.NewHealDelay`) 0.0)
    _))

(fn `TakeDamage`
  (params (Damage :type "Float (double-precision)") (DamageEvent :type "DamageEvent Structure (by ref)") (EventInstigator :type "Controller Object Reference") (DamageCauser :type "Actor Object Reference"))
  (returns (ReturnValue :type "Float (double-precision)"))
  (`self.SetHealDelay` Damage)
  (return Damage))