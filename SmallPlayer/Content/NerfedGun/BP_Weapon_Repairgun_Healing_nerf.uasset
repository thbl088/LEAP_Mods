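; Repair gun beam weapon component (nerf variant) that handles cosmetics for a beam locked onto a target.
; BeginPlay spawns two spline mesh actors for inner and outer beams, which Tick bends from muzzle to target, recoloring on team changes.
; Beam start/end events interpolate beam scale and material parameters and play heal or damage sounds based on target team.
; While the local player holds fire without a beam, searching sound and animation play.
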(event `self.ReceiveBeginPlay`
  (bind _innerspline (`self.InnerSpline`))
  (bind _outerspline (`self.OuterSpline`))
  (`/Engine/EditorBlueprintResources/StandardMacros.Can Execute Cosmetic Events`
    (:`True`
      (add `self.OnBeamStart` (`|CreateDelegate` :!event `OnBeamStartEvent`))
      (add `self.OnBeamEnd` (`|CreateDelegate` :!event `OnBeamEndEvent`))
      (`|ExecutionSequence`
        (:`then_0`
          (bind _returnvalue (`|SpawnActorFromClass` "/Script/Engine.SplineMeshActor" (`KismetMathLibrary.MakeTransform` (0.0 0.0 0.0)) "AlwaysSpawn" "OverrideRootScale" null null))
          (bind _output_get (set `self.InnerSpline` (`SplineMeshActor.SplineMeshComponent` _returnvalue)))
          (`SceneComponent.SetMobility` _output_get "Movable")
          (`StaticMeshComponent.SetStaticMesh` _innerspline "/Game/Art/Effects/Meshes/CylinderDivided.CylinderDivided")
          (`PrimitiveComponent.SetMaterial` _innerspline 0 "/Game/ThirdPartyAssets/LaserDamageVFX/Materials/ParticleMaterials/MI_RepairBeam.MI_RepairBeam")
          (`SceneComponent.SetMobility` _innerspline "Static")
          (`SceneComponent.SetVisibility` _innerspline false false)
          (`SplineMeshComponent.SetForwardAxis` _innerspline "Z" true)
          (`Actor.SetActorEnableCollision` (`self.GetOwner` _innerspline) false)
          (`PrimitiveComponent.SetCollisionResponseToAllChannels` _innerspline "ECR_Ignore")
          (`PrimitiveComponent.SetCollisionEnabled` _innerspline "NoCollision")
          (`PrimitiveComponent.SetCollisionResponseToAllChannels` _innerspline "ECR_Ignore"))
        (:`then_1`
          (bind _returnvalue_2 (`|SpawnActorFromClass` "/Script/Engine.SplineMeshActor" (`KismetMathLibrary.MakeTransform` (0.0 0.0 0.0)) "AlwaysSpawn" "OverrideRootScale" null null))
          (bind _output_get_2 (set `self.OuterSpline` (`SplineMeshActor.SplineMeshComponent` _returnvalue_2)))
          (`SceneComponent.SetMobility` _output_get_2 "Movable")
          (`StaticMeshComponent.SetStaticMesh` _outerspline "/Game/Art/Effects/Meshes/DoubleCylinderDivided_Smooth.DoubleCylinderDivided_Smooth")
          (`PrimitiveComponent.SetMaterial` _outerspline 0 "/Game/ThirdPartyAssets/LaserDamageVFX/Materials/ParticleMaterials/MI_RepairBeamOuter.MI_RepairBeamOuter")
          (`SceneComponent.SetMobility` _outerspline "Static")
          (`SceneComponent.SetVisibility` _outerspline false false)
          (`SplineMeshComponent.SetForwardAxis` _outerspline "Z" true)
          (`Actor.SetActorEnableCollision` (`self.GetOwner` _outerspline) false)
          (`PrimitiveComponent.SetCollisionResponseToAllChannels` _outerspline "ECR_Ignore")
          (`PrimitiveComponent.SetCollisionEnabled` _outerspline "NoCollision")
          (`PrimitiveComponent.SetCollisionResponseToAllChannels` _outerspline "ECR_Ignore"))))))

(event `self.ReceiveEndPlay`
  (params (EndPlayReason :type "EEndPlayReason Enum" :default "Destroyed"))
  (`parent.ReceiveEndPlay` EndPlayReason)
  (`|ExecutionSequence`
    (:`then_0`
      (if (`self.IsSplineValid`)
        (`self.K2_DestroyComponent` (`self.InnerSpline`))
        (`self.K2_DestroyComponent` (`self.OuterSpline`))))
    (:`then_1`
      (bind _loopingsound (`self.LoopingSound`)
        (:`then`
          (`self.K2_DestroyComponent` _loopingsound))
        (:`else`)))
    (:`then_2`
      (bind _searchingsound (`self.SearchingSound`)
        (:`then`
          (`self.K2_DestroyComponent` _searchingsound))
        (:`else`)))))

(event `OnBeamStartEvent` :!signature `self.OnBeamStart`
  (params (Mode :type Byte))
  (bind _returnvalue (`self.GetOwner`))
  (`|ExecutionSequence`
    (:`then_0`
      (`/Engine/EditorBlueprintResources/StandardMacros.IsValid` _returnvalue
        (:`Is Valid`
          (if (`|EnumEquality` (`Actor.GetLocalRole` _returnvalue) "ROLE_SimulatedProxy")
            (`self.SetComponentTickEnabled` true)
            (`self.RefreshBeamColor`)))))
    (:`then_1`
      (bind _weaponmesh (`self.GetWeaponMesh`))
      (`/Engine/EditorBlueprintResources/StandardMacros.IsValid` _weaponmesh
        (:`Is Valid`
          (`|ExecutionSequence`
            (:`then_0`
              (bind _issameteam (`self.IsSameTeam`))
              (bind _output_get (set `self.bIsTargetSameTeam` _issameteam))
              (if _output_get
                (`GameplayStatics.SpawnSoundAttached` "/Game/Audio/Weapons/RepairGun/RepairGun_Fire.RepairGun_Fire" _weaponmesh "Muzzle" (0.0 0.0 0.0) (struct) "SnapToTargetIncludingScale" false 1.0 1.0 0.0 null null)
                (else
                  (`GameplayStatics.SpawnSoundAttached` "/Game/Audio/Weapons/RepairGun/Damage_Beam_Activation.Damage_Beam_Activation" _weaponmesh "Muzzle" (0.0 0.0 0.0) (struct) "SnapToTargetIncludingScale" false 1.0 1.0 0.0 null null))))
            (:`then_1`
              (`self.LoopingSound`
                (:`then`
                  _)
                (:`else`
                  (if (`self.bIsTargetSameTeam`)
                    (bind _returnvalue_2 (`GameplayStatics.SpawnSoundAttached` "/Game/Audio/Weapons/RepairGun/RepairGun_Loop.RepairGun_Loop" _weaponmesh "Muzzle" (0.0 0.0 0.0) (struct) "SnapToTargetIncludingScale" false 1.0 1.0 0.0 null null false))
                    (bind _output_get_2 (set `self.LoopingSound` _returnvalue_2))
                    (else
                      (bind _returnvalue_3 (`GameplayStatics.SpawnSoundAttached` "/Game/Audio/Weapons/RepairGun/Damage_Beam_Loop.Damage_Beam_Loop" _weaponmesh "Muzzle" (0.0 0.0 0.0) (struct) "SnapToTargetIncludingScale" false 1.0 1.0 0.0 null null false))
                      (bind _output_get_3 (set `self.LoopingSound` _returnvalue_3))))))
              (`AudioComponent.FadeIn` _output_get_3 0.5 1.0 0.0 "Linear")
              (`AudioComponent.FadeIn` (`self.LoopingSound`) 0.5 1.0 0.0 "Linear")
              (`AudioComponent.FadeIn` _output_get_2 0.5 1.0 0.0 "Linear"))
            (:`then_2`
              (bind _asabp_weapon_repair_gun_1p (cast `/Game/Art/Weapons/Animations/RepairGun/1P/ABP_Weapon_RepairGun_1P` (`SkeletalMeshComponent.GetAnimInstance` _weaponmesh)))
              (bind _output_get_4 (set `/Game/Art/Weapons/Animations/RepairGun/1P/ABP_Weapon_RepairGun_1P.bIsRepairing` false _asabp_weapon_repair_gun_1p))
              (set `self.bIsRepairing` _output_get_4)
              (if (`self.IsSplineValid`)
                (`SplineMeshComponent.SetStartPosition` (`self.InnerSpline`) (`SceneComponent.GetSocketLocation` _weaponmesh "Muzzle") false)
                (`SplineMeshComponent.SetStartPosition` (`self.OuterSpline`) (`SceneComponent.GetSocketLocation` _weaponmesh "Muzzle") false)
                (`SplineMeshComponent.SetStartScale` (`self.InnerSpline`) (0.0 0.0) true)
                (`SplineMeshComponent.SetStartScale` (`self.OuterSpline`) (0.01 0.01) true)
                (`SceneComponent.SetVisibility` (`self.InnerSpline`) true false)
                (`SceneComponent.SetVisibility` (`self.OuterSpline`) true false)
                (`Interpolator.ClearInterpolatorsForObject` self)
                (bind _returnvalue_4 (`Interpolator.InterpolateOverTime` 0.0 1.0 0.0 1.0 "ExpoInOut" (`|CreateDelegate` :!event `BeamLatch`)))
                (set `self.BeamStartInterpolator` _returnvalue_4)))))))
    (:`then_2`
      (`/Engine/EditorBlueprintResources/StandardMacros.Can Execute Cosmetic Events`
        (:`True`
          (bind _searchingsound (`self.SearchingSound`)
            (:`then`
              (`AudioComponent.FadeOut` _searchingsound 1.0 0.0 "Linear")
              (`self.Toggle cosmeticTarget Seraching` false))
            (:`else`)))))
    (:`then_3`
      (`/Engine/EditorBlueprintResources/StandardMacros.Can Execute Cosmetic Events`
        (:`True`
          (if (`self.IsLocallyOwned`)
            (set `self.bHoldingTrigger` true)))))))

(event `OnBeamEndEvent` :!signature `self.OnBeamEnd`
  (params (Mode :type Byte))
  (bind _returnvalue (`self.GetOwner`))
  (`|ExecutionSequence`
    (:`then_0`
      (`/Engine/EditorBlueprintResources/StandardMacros.IsValid` _returnvalue
        (:`Is Valid`
          (if (`|EnumEquality` (`Actor.GetLocalRole` _returnvalue) "ROLE_SimulatedProxy")
            (`self.SetComponentTickEnabled` false)))))
    (:`then_1`
      (`self.KillLoopingSound`))
    (:`then_2`
      (if (`self.bIsRepairing`)
        (bind _weaponmesh (`self.GetWeaponMesh`))
        (`/Engine/EditorBlueprintResources/StandardMacros.IsValid` _weaponmesh
          (:`Is Valid`
            (`|ExecutionSequence`
              (:`then_0`
                (if (`self.bIsTargetSameTeam`)
                  (`GameplayStatics.SpawnSoundAttached` "/Game/Audio/Weapons/RepairGun/RepairGun_StopFire.RepairGun_StopFire" _weaponmesh "Muzzle" (0.0 0.0 0.0) (struct) "SnapToTargetIncludingScale" false 1.0 1.0 0.0 null null)
                  (else
                    (`GameplayStatics.SpawnSoundAttached` "/Game/Audio/Weapons/RepairGun/Damage_Beam_Complete.Damage_Beam_Complete" _weaponmesh "Muzzle" (0.0 0.0 0.0) (struct) "SnapToTargetIncludingScale" false 1.0 1.0 0.0 null null))))
              (:`then_1`
                (bind _asabp_weapon_repair_gun_1p (cast `/Game/Art/Weapons/Animations/RepairGun/1P/ABP_Weapon_RepairGun_1P` (`SkeletalMeshComponent.GetAnimInstance` _weaponmesh)))
                (bind _output_get (set `/Game/Art/Weapons/Animations/RepairGun/1P/ABP_Weapon_RepairGun_1P.bIsRepairing` false _asabp_weapon_repair_gun_1p))
                (set `self.bIsRepairing` _output_get)
                (if (`self.IsSplineValid`)
                  (`Interpolator.ClearInterpolatorsForObject` self)
                  (bind _returnvalue_2 (`Interpolator.InterpolateOverTime` 0.0 1.0 0.0 1.0 "ExpoInOut" (`|CreateDelegate` :!event `BeamLetGo`) (delegate `BeamEnd`)))
                  (set `self.BeamEndInterpolator` _returnvalue_2))))))))
    (:`then_3`
      (if (`self.bHoldingTrigger`)
        (`self.Cosmetically Search For Target`)))))

(event `KillLoopingSound`
  (bind _loopingsound (`self.LoopingSound`)
    (:`then`
      (`AudioComponent.FadeOut` _loopingsound 0.5 0.0 "Linear"))
    (:`else`)))

(event `BeamEnd`
  (params (Value :type "Float (double-precision)"))
  (`SceneComponent.SetVisibility` (`self.InnerSpline`) false false)
  (`SceneComponent.SetVisibility` (`self.OuterSpline`) false false))

(event `self.ReceiveTick`
  (params (DeltaSeconds :type "Float (single-precision)"))
  (bind _beamtargetactor (`self.BeamTargetActor`))
  (bind _outerspline (`self.OuterSpline`))
  (`/Engine/EditorBlueprintResources/StandardMacros.Can Execute Cosmetic Events`
    (:`True`
      (`|ExecutionSequence`
        (:`then_0`
          (`/Engine/EditorBlueprintResources/StandardMacros.IsValid` _beamtargetactor
            (:`Is Valid`
              (bind _returnvalue (message `TeamInterface.GetTeam` _beamtargetactor))
              (if (!= _returnvalue (`self.CachedTeam`))
                (set `self.CachedTeam` _returnvalue)
                (`self.RefreshBeamColor`)))
            (:`Is Not Valid`
              (set `self.CachedTeam` -1))))
        (:`then_1`
          (bind _weaponmesh (`self.GetWeaponMesh`))
          (`/Engine/EditorBlueprintResources/StandardMacros.IsValid` _weaponmesh
            (:`Is Valid`
              (if (`self.IsSplineValid`)
                (bind _returnvalue_location (`KismetMathLibrary.BreakTransform` (`SceneComponent.GetSocketTransform` _weaponmesh "Muzzle" "RTS_World")))
                (`SplineMeshComponent.SetStartPosition` _outerspline _returnvalue_location true)
                (`SplineMeshComponent.SetStartPosition` (`self.InnerSpline`) _returnvalue_location true)
                (bind _beamtargetactor_2 (`self.BeamTargetActor`)
                  (:`then`
                    (`SplineMeshComponent.SetStartTangent` _outerspline (* (`KismetMathLibrary.GetForwardVector` (`.OutRotation` (`Actor.GetActorEyesViewPoint` (`self.GetOwner`)))) 700.0) true)
                    (`SplineMeshComponent.SetStartTangent` (`self.InnerSpline`) (* (`KismetMathLibrary.GetForwardVector` (`.OutRotation` (`Actor.GetActorEyesViewPoint` (`self.GetOwner`)))) 700.0) true)
                    (bind _returnvalue_2 (`Actor.K2_GetActorLocation` _beamtargetactor_2))
                    (`SplineMeshComponent.SetEndTangent` _outerspline (* (`KismetMathLibrary.Normal` (- _returnvalue_2 _returnvalue_location)) 600.0) true)
                    (`SplineMeshComponent.SetEndTangent` (`self.InnerSpline`) (* (`KismetMathLibrary.Normal` (- _returnvalue_2 _returnvalue_location)) 600.0) true)
                    (`SplineMeshComponent.SetEndPosition` (`self.InnerSpline`) _returnvalue_2 true)
                    (`SplineMeshComponent.SetEndPosition` (`self.OuterSpline`) _returnvalue_2 true))
                  (:`else`))))))))))

(event `BeamLatch`
  (params (Value :type "Float (double-precision)"))
  (bind _returnvalue (`KismetMathLibrary.Lerp` 0.0 1.0 Value))
  (bind _returnvalue_2 (`KismetMathLibrary.Lerp` 0.0 1.2 Value))
  (if (`self.IsSplineValid`)
    (`SplineMeshComponent.SetEndScale` (`self.InnerSpline`) (`KismetMathLibrary.MakeVector2D` _returnvalue _returnvalue) true)
    (`SplineMeshComponent.SetEndScale` (`self.OuterSpline`) (`KismetMathLibrary.MakeVector2D` _returnvalue_2 _returnvalue_2) true)
    (`MeshComponent.SetScalarParameterValueOnMaterials` (`self.OuterSpline`) "Lines Tiling" (`KismetMathLibrary.MapRangeClamped` Value 0.0 1.0 0.0 10.0))
    (`MeshComponent.SetScalarParameterValueOnMaterials` (`self.OuterSpline`) "ScanLinesPower" (`KismetMathLibrary.MapRangeClamped` Value 0.0 1.0 200.0 5.0))))

(event `BeamLetGo`
  (params (Value :type "Float (double-precision)"))
  (bind _returnvalue (`KismetMathLibrary.Lerp` 1.0 0.0 Value))
  (bind _returnvalue_2 (`KismetMathLibrary.Lerp` 1.2 0.0 Value))
  (if (`self.IsSplineValid`)
    (`SplineMeshComponent.SetEndScale` (`self.InnerSpline`) (`KismetMathLibrary.MakeVector2D` _returnvalue _returnvalue) true)
    (`SplineMeshComponent.SetEndScale` (`self.OuterSpline`) (`KismetMathLibrary.MakeVector2D` _returnvalue_2 _returnvalue_2) true)
    (`MeshComponent.SetScalarParameterValueOnMaterials` (`self.OuterSpline`) "Lines Tiling" (`KismetMathLibrary.MapRangeClamped` Value 0.0 1.0 10.0))
    (`MeshComponent.SetScalarParameterValueOnMaterials` (`self.OuterSpline`) "ScanLinesPower" (`KismetMathLibrary.MapRangeClamped` Value 0.0 1.0 5.0 200.0))))

(event `RefreshBeamColor`
  (if (`self.IsSplineValid`)
    (`MeshComponent.SetVectorParameterValueOnMaterials` (`self.InnerSpline`) "BeamColor" (`KismetMathLibrary.Conv_LinearColorToVector` (`ProjectXGameState.GetTargetColour` (`self.BeamTargetActor`) "Healing" (`self.GetOwner`))))
    (`MeshComponent.SetVectorParameterValueOnMaterials` (`self.OuterSpline`) "BeamColor" (`KismetMathLibrary.Conv_LinearColorToVector` (`ProjectXGameState.GetTargetColour` (`self.BeamTargetActor`) "Healing" (`self.GetOwner`))))))

(event `Cosmetically Search For Target`
  (`/Engine/EditorBlueprintResources/StandardMacros.Can Execute Cosmetic Events` :!label _label
    (:`True`
      (if (`self.IsLocallyOwned`)
        (`WeaponComponent.CosmeticPrimaryFire` (`self.GetOwningComponent`))
        (set `self.bHoldingTrigger` true)
        (bind _searchingsound (`self.SearchingSound`)
          (:`then`
            (`AudioComponent.FadeIn` _searchingsound 1.0 1.0 0.0 "Linear"))
          (:`else`
            (bind _weaponmesh (`self.GetWeaponMesh`))
            (`/Engine/EditorBlueprintResources/StandardMacros.IsValid` _weaponmesh
              (:`Is Valid`
                (bind _returnvalue (`GameplayStatics.SpawnSoundAttached` "/Game/Audio/Weapons/RepairGun/RepairGunSearchingTarget_Loop.RepairGunSearchingTarget_Loop" _weaponmesh "Muzzle" (0.0 0.0 0.0) (struct) "SnapToTargetIncludingScale" true 1.0 1.0 0.0 null null false))
                (set `self.SearchingSound` _returnvalue)))))
        (`self.Toggle cosmeticTarget Seraching` true)))))

(event `self.K2_SearchingForTarget`
  (goto _label))

(event `self.K2_FireReleased`
  (params (Mode :type Byte))
  (`/Engine/EditorBlueprintResources/StandardMacros.Can Execute Cosmetic Events`
    (:`True`
      (if (`self.IsLocallyOwned`)
        (if (`self.bHoldingTrigger`)
          (`self.Toggle cosmeticTarget Seraching` false))
        (set `self.bHoldingTrigger` false)
        (bind _searchingsound (`self.SearchingSound`)
          (:`then`
            (`self.K2_DestroyComponent` _searchingsound))
          (:`else`))))))

(event `Toggle CosmeticTarget Seraching`
  (params (bToggle :type Boolean))
  (if (`self.IsLocallyOwned`)
    (`/Engine/EditorBlueprintResources/StandardMacros.Can Execute Cosmetic Events`
      (:`True`
        (`|ExecutionSequence`
          (:`then_0`
            (bind _weaponmesh (`self.GetWeaponMesh`))
            (`/Engine/EditorBlueprintResources/StandardMacros.IsValid` _weaponmesh
              (:`Is Valid`
                (bind _asabp_weapon_repair_gun_1p (cast `/Game/Art/Weapons/Animations/RepairGun/1P/ABP_Weapon_RepairGun_1P` (`SkeletalMeshComponent.GetAnimInstance` _weaponmesh)))
                (bind _output_get (set `/Game/Art/Weapons/Animations/RepairGun/1P/ABP_Weapon_RepairGun_1P.bIsTargetSearching` bToggle _asabp_weapon_repair_gun_1p))
                (`GameplayStatics.SpawnSoundAttached` (select `bool` _output_get :`false` "/Game/Audio/Weapons/RepairGun/RepairGun_StopTargetSearch.RepairGun_StopTargetSearch" :`true` "/Game/Audio/Weapons/RepairGun/RepairGun_StartTargetSearch.RepairGun_StartTargetSearch" :!type "SoundBase Object Reference") _weaponmesh "Muzzle" (0.0 0.0 0.0) (struct) "SnapToTargetIncludingScale" true 1.0 1.0 0.0 null null false))))
          (:`then_1`
            (`self.OnTargetSearching` bToggle)))))))

(event `self.K2_UnEquipComplete`
  (`parent.K2_UnEquipComplete`)
  (bind _searchingsound (`self.SearchingSound`)
    (:`then`
      (`AudioComponent.FadeOut` _searchingsound 0.2 0.0 "Linear"))
    (:`else`)))

(fn `GetWeaponMesh`
  (returns (WeaponMesh :type "SkeletalMeshComponent Object Reference"))
  (bind _returnvalue (`self.GetOwningComponent`))
  (`/Engine/EditorBlueprintResources/StandardMacros.IsValid` _returnvalue
    (:`Is Valid`
      (return (select `bool` (`|EnumEquality` (`Actor.GetLocalRole` (`self.GetOwner`)) "ROLE_SimulatedProxy") :`false` (`WeaponComponent.GetWeaponMesh1P` _returnvalue) :`true` (`WeaponComponent.GetWeaponMesh3P` _returnvalue))))
    (:`Is Not Valid`
      (return null))))

(fn `IsSameTeam`
  (returns (IsSameTeam :type Boolean))
  (if (== (`ProjectXGameState.GetTeamStatic` (`self.GetOwner`)) (`ProjectXGameState.GetTeamStatic` (`self.BeamTargetActor`)))
    (return true)
    (else
      (return false))))

(fn `IsSplineValid`
  (returns (IsValid :type Boolean))
  (return (and (`KismetSystemLibrary.IsValid` (`self.InnerSpline`)) (`KismetSystemLibrary.IsValid` (`self.OuterSpline`)))))