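; Deployable heal projector Blueprint, named as a nerfed Affliction ultimate variant, that handles the screen overlay shown while it is active.
; On Start, if the owning character is valid and locally controlled, it creates the heal projector overlay widget and adds it to the viewport.
; On End, it tells that widget to deactivate rather than removing it directly.
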(event `self.K2_Start`
  (bind _returnvalue (`self.GetOwningCharacter`))
  (`/Engine/EditorBlueprintResources/StandardMacros.IsValid` _returnvalue
    (:`Is Valid`
      (if (`Pawn.IsLocallyControlled` _returnvalue)
        (bind _returnvalue_2 (`|CreateWidget` "/Game/Blueprints/UI/W_HealProjectorOverlay.W_HealProjectorOverlay_C" (`GameplayStatics.GetPlayerController` 0)))
        (bind _output_get (set `self.Widget` _returnvalue_2))
        (`UserWidget.AddToViewport` _output_get 0)))))

(event `self.K2_End`
  (`/Engine/EditorBlueprintResources/StandardMacros.IsValid` (`self.Widget`)
    (:`Is Valid`
      (`/Game/Blueprints/UI/W_HealProjectorOverlay.Deactivate` (`self.Widget`)))))