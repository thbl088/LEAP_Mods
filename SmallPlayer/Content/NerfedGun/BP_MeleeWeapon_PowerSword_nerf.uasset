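; Power sword melee weapon Blueprint, mainly handling cosmetics for swings, reflection and equip state.
; Primary fire cycles montages, alternates the first-person animation pose and spawns four corner beams that Tick lerps toward the view's center line, plus an impact burst at maximum range.
; Reflection toggles the first-person AnimInstance's battle state for the owner and an attached Niagara trail for others.
; Equip starts a drone loop and delayed skin-aware blade particles, cleaned up on unequip.
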(event `self.ReceiveBeginPlay`
  (`/Engine/EditorBlueprintResources/StandardMacros.Can Execute Cosmetic Events`
    (:`True`
      (add `self.OnReflectionToggled` (delegate `ReflectionToggled`)))))

(event `ReflectionToggled` :!signature `self.OnReflectionToggled`
  (params (bToggle :type Boolean))
  (`self.ToggleBattleInstance` bToggle))

(event `ToggleBattleInstance`
  (params (bToggle :type Boolean))
  (bind _returnvalue (`self.GetOwningCharacter`))
  (bind _cachedaniminstance (`self.CachedAnimInstance`))
  (bind _reflectsystem (`self.ReflectSystem`))
  (bind _returnvalue_2 (`ProjectXCharacter.GetCosmeticsComponent` _returnvalue))
  (`/Engine/EditorBlueprintResources/StandardMacros.Can Execute Cosmetic Events`
    (:`True`
      (if (`self.IsLocallyOwned`)
        (`/Engine/EditorBlueprintResources/StandardMacros.IsValid` _returnvalue
          (:`Is Valid`
            (`/Engine/EditorBlueprintResources/StandardMacros.IsValid` _returnvalue_2
              (:`Is Valid`
                (`|ExecutionSequence`
                  (:`then_0`
                    (bind _mesh1p (`CosmeticsComponent.Mesh1P` _returnvalue_2)
                      (:`then`
                        (bind _returnvalue_3 (`SkeletalMeshComponent.GetAnimInstance` _mesh1p))
                        (`/Engine/EditorBlueprintResources/StandardMacros.IsValid` _returnvalue_3
                          (:`Is Valid`
                            (bind _asabp_character_first_person_v3 (cast `/Game/Art/Characters/Animations/Default/FP/ABP_Character_FirstPerson_V3` _returnvalue_3)
                              (:`then`
                                (bind _output_get (set `self.CachedAnimInstance` _asabp_character_first_person_v3))
                                (`/Game/Art/Characters/Animations/Default/FP/ABP_Character_FirstPerson_V3.SetTightAimAsAlt` _output_get true)
                                (if bToggle
                                  (`/Game/Art/Characters/Animations/Default/FP/ABP_Character_FirstPerson_V3.ToggleBattleInstance` _cachedaniminstance true)
                                  (else
                                    (`/Game/Art/Characters/Animations/Default/FP/ABP_Character_FirstPerson_V3.ToggleBattleInstance` _cachedaniminstance false)))
                                (`KismetSystemLibrary.K2_ClearAndInvalidateTimerHandle` (`self.BattleInstanceTimerHandle`)))
                              (:`CastFailed`
                                (bind _cachedaniminstance_2 (`self.CachedAnimInstance` :!label _label)
                                  (:`then`
                                    (`/Game/Art/Characters/Animations/Default/FP/ABP_Character_FirstPerson_V3.ToggleBattleInstance` _cachedaniminstance_2 false)
                                    (set `self.CachedAnimInstance` null)
                                    (`KismetSystemLibrary.K2_ClearAndInvalidateTimerHandle` (`self.BattleInstanceTimerHandle`)))
                                  (:`else`)))))
                          (:`Is Not Valid`
                            (goto _label))))
                      (:`else`
                        (goto _label))))))
              (:`Is Not Valid`
                (goto _label))))
          (:`Is Not Valid`
            (goto _label)))
        (elif bToggle
          (`/Engine/EditorBlueprintResources/StandardMacros.IsValid` _reflectsystem
            (:`Is Valid`
              (`self.Activate` _reflectsystem true))
            (:`Is Not Valid`
              (bind _returnvalue_4 (`NiagaraFunctionLibrary.SpawnSystemAttached` "/Game/ThirdPartyAssets/EssentialVFXPackV1/NiagaraVFX/NS_BubbleTrail.NS_BubbleTrail" (`Actor.RootComponent` _returnvalue) "None" (0.0 0.0 0.0) (struct) "KeepRelativeOffset"))
              (set `self.ReflectSystem` _returnvalue_4)))
          (else
            (`/Engine/EditorBlueprintResources/StandardMacros.IsValid` _reflectsystem
              (:`Is Valid`
                (`self.Deactivate` (`self.ReflectSystem`))))))))))

(event `self.K2_Equip`
  (`/Engine/EditorBlueprintResources/StandardMacros.Can Execute Cosmetic Events`
    (:`True`
      (bind _returnvalue (`GameplayStatics.SpawnSoundAttached` "/Game/Audio/Weapons/Sword/MACK_Drone_Low_Resonate_LOOP_Cue.MACK_Drone_Low_Resonate_LOOP_Cue" (`Actor.RootComponent` (`self.GetOwner`)) "None" (0.0 0.0 0.0) (struct) "KeepRelativeOffset" false 1.0 1.0 0.0 null null))
      (set `self.DroneSound` _returnvalue)
      (`self.SpawnWeaponParticles`)
      (`self.ToggleBattleInstance` false))))

(event `self.K2_UnEquip`
  (`|ExecutionSequence` :!label _label_2
    (:`then_0`
      (`self.ToggleBattleInstance` false))
    (:`then_1`
      (`/Engine/EditorBlueprintResources/StandardMacros.IsValid` (`self.DroneSound`)
        (:`Is Valid`
          (`AudioComponent.FadeOut` (`self.DroneSound`) 0.5 0.0 "Linear"))))
    (:`then_2`
      (`/Engine/EditorBlueprintResources/StandardMacros.IsValid` (`self.SwordParticles`)
        (:`Is Valid`
          (`self.K2_DestroyComponent` (`self.SwordParticles`)))))))

(event `self.ReceiveEndPlay`
  (params (EndPlayReason :type "EEndPlayReason Enum" :default "Destroyed"))
  (goto _label_2))

(event `self.K2_Fire`
  (params (Mode :type Byte))
  (bind _customclambermontages (`self.CustomClamberMontages`))
  (bind _meleeextent (`self.MeleeExtent`))
  (bind _meleeextent_2 (`self.MeleeExtent`))
  (bind _returnvalue (`KismetMathLibrary.Conv_ByteToInt` (`self.AnimCounter`)))
  (bind (_outlocation _outrotation) (`Actor.GetActorEyesViewPoint` (`self.GetOwner`)))
  (bind _returnvalue_2 (* _meleeextent -1.0))
  (bind _returnvalue_3 (* _meleeextent_2 -1.0 (`KismetMathLibrary.SelectFloat` 1.0 0.25 (`self.IsLocallyOwned`))))
  (bind _output (`|GetArrayItem` _customclambermontages _returnvalue))
  (bind _returnvalue_4 (* (`KismetMathLibrary.GetUpVector` _outrotation) _returnvalue_2))
  (bind _returnvalue_5 (* (`KismetMathLibrary.GetRightVector` _outrotation) _returnvalue_2))
  (bind _returnvalue_6 (* (`KismetMathLibrary.GetRightVector` _outrotation) _meleeextent))
  (bind _returnvalue_7 (* (`KismetMathLibrary.GetUpVector` _outrotation) _meleeextent))
  (bind _returnvalue_8 (* (`KismetMathLibrary.GetRightVector` _outrotation) _meleeextent_2))
  (bind _returnvalue_9 (* (`KismetMathLibrary.GetUpVector` _outrotation) _meleeextent_2))
  (bind _returnvalue_10 (* (`KismetMathLibrary.GetRightVector` _outrotation) _returnvalue_3))
  (bind _returnvalue_11 (* (`KismetMathLibrary.GetUpVector` _outrotation) _returnvalue_3))
  (bind _returnvalue_12 (`KismetMathLibrary.SelectVector` _outlocation (+ (`SceneComponent.GetSocketLocation` (`WeaponComponent.GetMesh3P` (`self.GetOwningComponent`)) "spine_03") (* (`KismetMathLibrary.GetForwardVector` _outrotation) 150.0)) (`self.IsLocallyOwned`)))
  (bind _returnvalue_13 (+ _returnvalue_12 _returnvalue_10 _returnvalue_11))
  (bind _returnvalue_14 (+ _returnvalue_12 (* (`KismetMathLibrary.GetForwardVector` _outrotation) (`self.MeleeRange`))))
  (bind _returnvalue_15 (+ _returnvalue_12 _returnvalue_8 _returnvalue_9))
  (bind _returnvalue_16 (+ _returnvalue_12 _returnvalue_10 _returnvalue_9))
  (bind _returnvalue_17 (+ _returnvalue_12 _returnvalue_8 _returnvalue_11))
  (`/Engine/EditorBlueprintResources/StandardMacros.Can Execute Cosmetic Events`
    (:`True`
      (if (== Mode 0)
        (`|ExecutionSequence`
          (:`then_0`
            (`self.SetFireAnimMontage` (`|GetArrayItem` (`self.CustomFireAnimMontages`) (`KismetMathLibrary.Conv_ByteToInt` (`self.AnimCounter`))) (`|GetArrayItem` (`self.CustomFireAnimMontages3P`) (`KismetMathLibrary.Conv_ByteToInt` (`self.AnimCounter`))))
            (set `self.ToggledInstance` (not (`self.ToggledInstance`)))
            (set `self.AnimCounter` (+ (`self.AnimCounter`) 1))
            (set `self.AnimCounter` (select `bool` (`KismetArrayLibrary.Array_IsValidIndex` (select `bool` (`self.IsLocallyOwned`) :`false` (`self.CustomFireAnimMontages3P`) :`true` (`self.CustomFireAnimMontages`)) (`KismetMathLibrary.Conv_ByteToInt` (`self.AnimCounter`))) :`true` (`self.AnimCounter`)))
            (bind _cachedaniminstance (`self.CachedAnimInstance`)
              (:`then`
                (`/Game/Art/Characters/Animations/Default/FP/ABP_Character_FirstPerson_V3.ToggleTightAimManual` _cachedaniminstance (`self.ToggledInstance`))
                (if (`KismetArrayLibrary.Array_IsValidIndex` _customclambermontages _returnvalue)
                  (`/Engine/EditorBlueprintResources/StandardMacros.IsValid` _output
                    (:`Is Valid`
                      (`/Game/Art/Characters/Animations/Default/FP/ABP_Character_FirstPerson_V3.SetClamberMontage` _cachedaniminstance (select `bool` (`self.ToggledInstance`) :`false` _output :`true` "/Game/Art/Characters/Animations/FusionBlade/1P/Hands_Blade_Clamber3_Montage.Hands_Blade_Clamber3_Montage"))))))
              (:`else`)))
          (:`then_1`
            (`KismetArrayLibrary.Array_Clear` (`self.BeamParticles`))
            (set `self.CachedSourcelocation` _returnvalue_12)
            (set `self.CachedTargetLocation` _returnvalue_14)
            (bind _returnvalue_18 (`GameplayStatics.SpawnEmitterAtLocation` "/Game/Art/Effects/BeamAndLaserFX01/Particles/P_ky_beam02.P_ky_beam02" _returnvalue_15 (struct) (1.0 1.0 1.0) true "AutoRelease" true 625000000.0 (not (`self.IsLocallyOwned`))))
            (`/Engine/EditorBlueprintResources/StandardMacros.IsValid` _returnvalue_18
              (:`Is Valid`
                (`KismetArrayLibrary.Array_Add` (`self.BeamParticles`) _returnvalue_18)
                (`ParticleSystemComponent.SetBeamSourcePoint` _returnvalue_18 0 _returnvalue_15 0)
                (`ParticleSystemComponent.SetBeamTargetPoint` _returnvalue_18 0 (+ _returnvalue_14 _returnvalue_6 _returnvalue_7) 0)
                (bind _returnvalue_19 (`GameplayStatics.SpawnEmitterAtLocation` "/Game/Art/Effects/BeamAndLaserFX01/Particles/P_ky_beam02.P_ky_beam02" _returnvalue_16 (struct) (1.0 1.0 1.0) true "AutoRelease" true 625000000.0 (not (`self.IsLocallyOwned`))))
                (`/Engine/EditorBlueprintResources/StandardMacros.IsValid` _returnvalue_19
                  (:`Is Valid`
                    (`KismetArrayLibrary.Array_Add` (`self.BeamParticles`) _returnvalue_19)
                    (`ParticleSystemComponent.SetBeamSourcePoint` _returnvalue_19 0 _returnvalue_16 0)
                    (`ParticleSystemComponent.SetBeamTargetPoint` _returnvalue_19 0 (+ _returnvalue_14 _returnvalue_5 _returnvalue_7) 0))
                  (:`Is Not Valid`
                    _))
                (bind _returnvalue_20 (`GameplayStatics.SpawnEmitterAtLocation` "/Game/Art/Effects/BeamAndLaserFX01/Particles/P_ky_beam02.P_ky_beam02" _returnvalue_17 (struct) (1.0 1.0 1.0) true "AutoRelease" true 625000000.0 (not (`self.IsLocallyOwned`))))
                (`/Engine/EditorBlueprintResources/StandardMacros.IsValid` _returnvalue_20
                  (:`Is Valid`
                    (`KismetArrayLibrary.Array_Add` (`self.BeamParticles`) _returnvalue_20)
                    (`ParticleSystemComponent.SetBeamSourcePoint` _returnvalue_20 0 _returnvalue_17 0)
                    (`ParticleSystemComponent.SetBeamTargetPoint` _returnvalue_20 0 (+ _returnvalue_14 _returnvalue_6 _returnvalue_4) 0))
                  (:`Is Not Valid`
                    _))
                (bind _returnvalue_21 (`GameplayStatics.SpawnEmitterAtLocation` "/Game/Art/Effects/BeamAndLaserFX01/Particles/P_ky_beam02.P_ky_beam02" _returnvalue_13 (struct) (1.0 1.0 1.0) true "AutoRelease" true 625000000.0 (not (`self.IsLocallyOwned`))))
                (`/Engine/EditorBlueprintResources/StandardMacros.IsValid` _returnvalue_21
                  (:`Is Valid`
                    (`KismetArrayLibrary.Array_Add` (`self.BeamParticles`) _returnvalue_21)
                    (`ParticleSystemComponent.SetBeamSourcePoint` _returnvalue_21 0 _returnvalue_13 0)
                    (`ParticleSystemComponent.SetBeamTargetPoint` _returnvalue_21 0 (+ _returnvalue_14 _returnvalue_5 _returnvalue_4) 0))
                  (:`Is Not Valid`
                    _))
                (`|ExecutionSequence`
                  (:`then_0`
                    (`KismetSystemLibrary.Delay` (`self.GetFireRate`))
                    (`KismetArrayLibrary.Array_Clear` (`self.BeamParticles`)))
                  (:`then_1`
                    (`GameplayStatics.SpawnEmitterAtLocation` "/Game/Art/Effects/Particles/BulletImpacts/Deprecated/PS_Impact_Electrical_Large.PS_Impact_Electrical_Large" (`self.CachedTargetLocation`))))))))))))

(event `self.ReceiveTick`
  (params (DeltaSeconds :type "Float (single-precision)"))
  (bind _returnvalue (* DeltaSeconds (`KismetMathLibrary.SelectFloat` 3.0 6.0 (`self.IsLocallyOwned`))))
  (for _array_element (`self.BeamParticles`)
    (`/Engine/EditorBlueprintResources/StandardMacros.IsValid` _array_element
      (:`Is Valid`
        (`ParticleSystemComponent.SetBeamSourcePoint` _array_element 0 (`KismetMathLibrary.VLerp` (`ParticleSystemComponent.GetBeamSourcePoint` _array_element 0 0) (`self.CachedSourcelocation`) _returnvalue) 0)
        (`ParticleSystemComponent.SetBeamTargetPoint` _array_element 0 (`KismetMathLibrary.VLerp` (`ParticleSystemComponent.GetBeamTargetPoint` _array_element 0 0) (`self.CachedTargetLocation`) _returnvalue) 0)))))

(event `self.K2_FireReleased`
  (params (Mode :type Byte))
  (`/Engine/EditorBlueprintResources/StandardMacros.Can Execute Cosmetic Events`
    (:`True`
      (if (not (== Mode 0))
        (`self.ToggleBattleInstance` false)))))

(event `self.OnWeaponParticleLoaded`
  (params (Particle :type "ParticleSystem Object Reference"))
  (`/Engine/EditorBlueprintResources/StandardMacros.IsValid` Particle
    (:`Is Valid`
      (`self.SpawnWeaponParticles`))))

(event `SpawnWeaponParticles`
  (bind _returnvalue (`self.GetOwningComponent`))
  (`/Engine/EditorBlueprintResources/StandardMacros.IsValid` (`self.SwordParticles`)
    (:`Is Valid`
      (`self.K2_DestroyComponent` (`self.SwordParticles`)))
    (:`Is Not Valid`
      _))
  (`KismetSystemLibrary.Delay` 1.0)
  (if (and (`WeaponComponent.IsCurrentWeapon` (`self.GetOwningComponent`) self) (not (`self.IsUnEquipping`)))
    (bind _returnvalue_2 (`GameplayStatics.SpawnEmitterAttached` (select `bool` (`KismetSystemLibrary.IsValid` (`self.WeaponSkinParticle`)) :`false` "/Game/Art/Weapons/Materials/FusionBlade/Effect/P_FusionSword_Skin01.P_FusionSword_Skin01" :`true` (`self.WeaponSkinParticle`)) (select `bool` (`self.IsLocallyOwned`) :`false` (`WeaponComponent.GetWeaponMesh3P` _returnvalue) :`true` (`WeaponComponent.GetWeaponMesh1P` _returnvalue) :!type "SceneComponent Object Reference") "sword_base" (0.0 1.0 0.0)))
    (set `self.SwordParticles` _returnvalue_2)))

(fn `GetAnimState`
  (returns (ReturnValue :type Integer))
  (return (`KismetMathLibrary.SelectInt` 2 (`KismetMathLibrary.Conv_ByteToInt` (`self.AnimCounter`)) (`self.ToggledInstance`))))