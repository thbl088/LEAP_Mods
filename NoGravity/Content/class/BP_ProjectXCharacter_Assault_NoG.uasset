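; Assault character variant that equips the NoG version of the impact grenade as its secondary ability.
; After a short delay on BeginPlay, it caches primary and secondary weapons and abilities from the WeaponComponent slots.
; It then adds the grenade to the secondary ability slot regardless of the current one, as the impact grenade check has empty branches.
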(event `self.ReceiveBeginPlay`
  (`parent.ReceiveBeginPlay`)
  (`KismetSystemLibrary.Delay` 0.2)
  (`self.SetWeapons`)
  (if (== (`self.SecondaryAbilityPlayer`) "/Game/Blueprints/Weapons/BP_Weapon_ImpactGrenade.BP_Weapon_ImpactGrenade")
    _
    (else
      _))
  (`WeaponComponent.AddWeapon` (`self.WeaponComponent`) "/NoGravity/projectiles/Assault/BP_Weapon_ImpactGrenade_NoG.BP_Weapon_ImpactGrenade_NoG_C" "SecondaryAbility" false))

(fn `SetWeapons`
  (bind _weaponcomponent (`self.WeaponComponent`))
  (set `self.PrimWeapon` (`WeaponComponent.GetWeaponFromSlot` _weaponcomponent "PrimaryWeapon"))
  (set `self.SecWeapon` (`WeaponComponent.GetWeaponFromSlot` _weaponcomponent "SecondaryWeapon"))
  (set `self.PrimAbilitiy` (`WeaponComponent.GetWeaponFromSlot` _weaponcomponent "PrimaryAbility"))
  (set `self.SecondaryAbilityPlayer` (`WeaponComponent.GetWeaponFromSlot` _weaponcomponent "SecondaryAbility")))

(fn `UserConstructionScript`
  (`parent.UserConstructionScript`))