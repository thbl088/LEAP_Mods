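; Deployable Sonic Projector: a thrown device that deploys where it first hits, then gives off sonic pulses until its lifetime expires.
; The server handles the hit and activates the AfflictionVolume on deploy; cosmetic-capable instances play landing, shell-opening and team-colour effects.
; Tick drives core spin and pulses of EMP particles, camera shake, glow and increasingly loud, higher-pitched sound.
; Death triggers an explosion and dissolves the meshes through a dynamic material.
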(event `self.ReceiveBeginPlay`
  (bind _projectorroot (`self.ProjectorRoot`))
  (bind (_returnvalue_roll _returnvalue_pitch _returnvalue_yaw) (`KismetMathLibrary.BreakRotator` (`SceneComponent.K2_GetComponentRotation` _projectorroot)))
  (`|ExecutionSequence`
    (:`then_0`
      (`/Engine/EditorBlueprintResources/StandardMacros.Can Execute Cosmetic Events`
        (:`True`
          (bind _returnvalue (`GameplayStatics.SpawnSoundAttached` "/Game/Audio/Weapons/SonicProjector/SonicProjector_StartUp_Cue.SonicProjector_StartUp_Cue" (`self.SphereRoot`) "None" (0.0 0.0 0.0) (struct) "SnapToTargetIncludingScale" true 3.0 1.0 0.0 null null))
          (set `self.GeneratorLoop` _returnvalue)
          (`Interpolator.InterpolateOverTimeSimple` 3.0 "EaseIn" (delegate `Core Rotate Ramp Up`))
          (`Interpolator.InterpolateOverTimeSimple` 4.0 "ExpoOut" (delegate `Throw Rotate`)))
        (:`False`
          (`|ExecutionSequence`
            (:`then_0`
              (bind _afterburner (`self.Afterburner`)
                (:`then`
                  (`ActorComponent.K2_DestroyComponent` _afterburner))
                (:`else`)))
            (:`then_1`
              (bind _afterburner1 (`self.Afterburner1`)
                (:`then`
                  (`ActorComponent.K2_DestroyComponent` _afterburner1))
                (:`else`)))
            (:`then_2`
              (bind _afterburner3 (`self.Afterburner3`)
                (:`then`
                  (`ActorComponent.K2_DestroyComponent` _afterburner3))
                (:`else`)))
            (:`then_3`
              (bind _afterburner4 (`self.Afterburner4`)
                (:`then`
                  (`ActorComponent.K2_DestroyComponent` _afterburner4))
                (:`else`)))))))
    (:`then_1`
      (`SceneComponent.K2_SetWorldRotation` _projectorroot (`KismetMathLibrary.MakeRotator` _returnvalue_roll 0.0 _returnvalue_yaw) false false))))

(event `Core Rotate Ramp Up`
  (params (Value :type "Float (double-precision)"))
  (set `self.CoreRotationRate` (* Value 30.0)))

(event `Throw Rotate`
  (params (Value :type "Float (double-precision)"))
  (bind _projectorroot (`self.ProjectorRoot`)
    (:`then`
      (`SceneComponent.K2_AddLocalRotation` _projectorroot (`KismetMathLibrary.MakeRotator` 0.0 0.0 (`KismetMathLibrary.Lerp` 12.0 0.0 Value)) false false))
    (:`else`)))

(event `self.ReceiveHit`
  (params (MyComp :type "PrimitiveComponent Object Reference") (Other :type "Actor Object Reference") (OtherComp :type "PrimitiveComponent Object Reference") (bSelfMoved :type Boolean) (HitLocation :type "Vector Structure") (HitNormal :type "Vector Structure") (NormalImpulse :type "Vector Structure") (Hit :type "HitResult Structure (by ref)"))
  (`/Engine/EditorBlueprintResources/ActorMacros.Switch Has Authority`
    (:`Authority`
      (`/Engine/EditorBlueprintResources/StandardMacros.DoOnce` false
        (:`Completed`
          (`self.DeployStart` true)
          (`self.K2_SetActorLocation` (`.Location` (`GameplayStatics.BreakHitResult` Hit))))))))

(event `self.OnDeployComplete`
  (bind _returnvalue (`self.K2_GetActorLocation`))
  (bind _returnvalue_2 (`SceneComponent.K2_GetComponentLocation` (`self.ProjectorRoot`)))
  (`self.SetActorTickEnabled` true)
  (`|ExecutionSequence`
    (:`then_0`
      (`/Engine/EditorBlueprintResources/ActorMacros.Switch Has Authority`
        (:`Authority`
          (`ActorComponent.Activate` (`self.AfflictionVolume`) false))))
    (:`then_1`
      (`/Engine/EditorBlueprintResources/StandardMacros.Can Execute Cosmetic Events`
        (:`True`
          (`self.TeamColour`))))
    (:`then_2`
      (`/Engine/EditorBlueprintResources/StandardMacros.Can Execute Cosmetic Events`
        (:`True`
          (`GameplayStatics.PlayWorldCameraShake` "/Game/Blueprints/Weapons/Deployable/Deployables/Containers/BP_ContainerLandShake.BP_ContainerLandShake_C" (`self.K2_GetActorLocation`) 1000.0 5000.0)
          (`GameplayStatics.PlaySoundAtLocation` "/Game/Audio/Deployables/Containers/ContainerImpact_Cue.ContainerImpact_Cue" _returnvalue (struct) 1.0 1.0 0.0 null null null)
          (`GameplayStatics.SpawnEmitterAtLocation` "/Game/Art/Effects/Particles/BulletImpacts/Deprecated/PS_Impact_Deployable.PS_Impact_Deployable" _returnvalue)
          (bind _returnvalue_3 (`GameplayStatics.SpawnEmitterAttached` "/Game/Art/Effects/Particles/Trails/PS_DeployableTrail.PS_DeployableTrail" (`self.RootComponent`)))
          (set `self.DeployTrail` _returnvalue_3)
          (`KismetSystemLibrary.Delay` 0.1)
          (bind _deploytrail (`self.DeployTrail`)
            (:`then`
              (`ActorComponent.Deactivate` _deploytrail))
            (:`else`)))))
    (:`then_3`
      (`/Engine/EditorBlueprintResources/StandardMacros.Can Execute Cosmetic Events`
        (:`True`
          (`|ExecutionSequence`
            (:`then_0`
              (`GameplayStatics.SpawnEmitterAtLocation` "/Game/ThirdPartyAssets/FireEnergyVFX/Particles/P_Appear1.P_Appear1" _returnvalue_2)
              (`GameplayStatics.PlaySoundAtLocation` "/Game/Audio/Weapons/HealProjector/emit_Cue.emit_Cue" _returnvalue_2 (struct) 1.0 1.0 0.0 null null null)
              (bind _returnvalue_4 (`GameplayStatics.SpawnEmitterAttached` "/Game/ThirdPartyAssets/FireEnergyVFX/Particles/P_Portal1.P_Portal1" (`self.Sonic Projector Core`) "None" (0.0 0.0 0.0) (struct) (1.0 1.0 1.0) "SnapToTarget"))
              (set `self.LoopingParticleSystem` _returnvalue_4)
              (`Interpolator.InterpolateOverTimeSimple` 1.0 "EaseOut" (delegate `Open Shell`)))
            (:`then_1`
              (`Interpolator.InterpolateOverTimeSimple` 5.0 "ExpoOut" (delegate `Landed`)))))))))

(event `self.OnDeployStart`
  (`self.SetActorEnableCollision` true))

(event `Open Shell`
  (params (Value :type "Float (double-precision)"))
  (bind _returnvalue (`KismetMathLibrary.Lerp` 0.0 30.0 Value))
  (bind _sonic_projector_shell (`self.Sonic Projector Shell`)
    (:`then`
      (`SceneComponent.K2_SetRelativeLocation` _sonic_projector_shell (`KismetMathLibrary.MakeVector` 0.0 _returnvalue) false false)
      (bind _sonic_projector_shell1 (`self.Sonic Projector Shell1`)
        (:`then`
          (`SceneComponent.K2_SetRelativeLocation` _sonic_projector_shell1 (`KismetMathLibrary.MakeVector` 0.0 (* _returnvalue -1.0)) false false))
        (:`else`)))
    (:`else`)))

(event `Landed`
  (params (Value :type "Float (double-precision)"))
  (`SceneComponent.K2_SetRelativeLocation` (`self.ProjectorRoot`) (`KismetMathLibrary.MakeVector` 0.0 0.0 (* (`KismetMathLibrary.DegSin` (`KismetMathLibrary.Lerp` 0.0 720.0 Value)) (- 1.0 Value) -25.0)) false false))

(event `self.ReceiveTick`
  (params (DeltaSeconds :type "Float (single-precision)"))
  (bind _returnvalue (`self.K2_GetActorLocation`))
  (bind _returnvalue_2 (+ DeltaSeconds (`self.Increment`)))
  (if (not (`HealthInterface.IsDead`))
    (`|ExecutionSequence`
      (:`then_0`
        (if (`self.First?`)
          (set `self.First?` false)
          (`KismetSystemLibrary.Delay` (`self.DeployTime`)))
        (if (<= (- (`self.Increment`) (+ (`self.landTime`) (`self.DeployTime`))) (`self.DeployableLifeTime`))
          (`|ExecutionSequence`
            (:`then_0`
              (`/Engine/EditorBlueprintResources/StandardMacros.Can Execute Cosmetic Events`
                (:`True`
                  (`GameplayStatics.PlaySoundAtLocation` "/Game/Audio/Explosions/SciFi/Mountain_Audio_-_Laser_Hit_Explosion_Cue.Mountain_Audio_-_Laser_Hit_Explosion_Cue" _returnvalue (struct) (/ _returnvalue_2 3.0) (* _returnvalue_2 0.208) 0.0 null null null)
                  (`GameplayStatics.SpawnEmitterAtLocation` (select `bool` (`ProjectXGameState.IsAlly` (`self.GetOwner`) (`GameplayStatics.GetPlayerController` 0)) :`false` "/Game/Art/Effects/Particles/Explosions/P_EMP.P_EMP" :`true` "/Game/Art/Effects/Particles/Explosions/P_EMP_ALly.P_EMP_Ally" :!type "ParticleSystem Object Reference") _returnvalue)
                  (`Interpolator.InterpolateOverTime` 0.0 1.0 0.0 1.0 "EaseOut" (delegate `Pulse`))
                  (`GameplayStatics.PlayWorldCameraShake` "/Game/ThirdPartyAssets/IBFPSStarterPack/Blueprints/BP_SonicCameraShake.BP_SonicCameraShake_C" (`self.K2_GetActorLocation`) 1000.0 6000.0 10.0))))
            (:`then_1`
              (set `self.Increment` _returnvalue_2)))))
      (:`then_1`
        (`/Engine/EditorBlueprintResources/StandardMacros.Can Execute Cosmetic Events`
          (:`True`
            (`Interpolator.InterpolateOverTime` 0.0 1.0 0.0 1.0 "Linear" (delegate `Rotate Core`))))))))

(event `Pulse`
  (params (Value :type "Float (double-precision)"))
  (bind _returnvalue (`KismetMathLibrary.DegSin` (`KismetMathLibrary.Lerp` 0.0 180.0 Value)))
  (bind _sonic_projector_core (`self.Sonic Projector Core`)
    (:`then`
      (`MeshComponent.SetScalarParameterValueOnMaterials` _sonic_projector_core "EmissiveStrength" (`KismetMathLibrary.Lerp` 0.0 50.0 _returnvalue))
      (bind _pointlight (`self.PointLight`)
        (:`then`
          (`LightComponent.SetIntensity` _pointlight (`KismetMathLibrary.Lerp` 1000.0 50000.0 _returnvalue)))
        (:`else`)))
    (:`else`)))

(event `Rotate Core`
  (params (Value :type "Float (double-precision)"))
  (bind _corerotationrate (`self.CoreRotationRate`))
  (bind _sonic_projector_core (`self.Sonic Projector Core`)
    (:`then`
      (`SceneComponent.K2_AddLocalRotation` _sonic_projector_core (`KismetMathLibrary.MakeRotator` 0.0 _corerotationrate (/ _corerotationrate 3.0)) false true))
    (:`else`)))

(event `TeamColour`
  (bind _returnvalue (`KismetMathLibrary.SelectColor` (struct :`G` 0.7 :`B` 0.8 :`A` 1.0) (struct :`R` 0.83 :`G` 0.4 :`A` 1.0) (`ProjectXGameState.IsAlly` self (`GameplayStatics.GetPlayerController` 0))))
  (bind _pointlight (`self.PointLight` :!label _label)
    (:`then`
      (`LightComponent.SetLightColor` _pointlight _returnvalue true))
    (:`else`
      _))
  (bind _sonic_projector_core (`self.Sonic Projector Core`)
    (:`then`
      (`MeshComponent.SetVectorParameterValueOnMaterials` _sonic_projector_core "Emissive Colour" (`KismetMathLibrary.Conv_LinearColorToVector` _returnvalue))
      (`MeshComponent.SetVectorParameterValueOnMaterials` (`self.Sonic Projector Shell1`) "Emissive Colour" (`KismetMathLibrary.Conv_LinearColorToVector` _returnvalue))
      (`MeshComponent.SetVectorParameterValueOnMaterials` (`self.Sonic Projector Shell`) "Emissive Colour" (`KismetMathLibrary.Conv_LinearColorToVector` _returnvalue)))
    (:`else`)))

(event `self.InitializeForTeam`
  (params (Team :type Integer))
  (set `self.Team` Team)
  (set `self.bIsAlly` (`ProjectXGameState.IsAlly` self (`GameplayStatics.GetPlayerController` 0)))
  (goto _label))

(event `self.OnDeployDeactivated`
  (`/Engine/EditorBlueprintResources/StandardMacros.Can Execute Cosmetic Events`
    (:`True`
      (set `self.Deactivated` true :!label _label_2)
      (bind _generatorloop (`self.GeneratorLoop`)
        (:`then`
          (`AudioComponent.FadeOut` _generatorloop 0.5 0.0 "Linear"))
        (:`else`
          _))
      (bind _loopingparticlesystem (`self.LoopingParticleSystem`)
        (:`then`
          (`ActorComponent.Deactivate` _loopingparticlesystem))
        (:`else`)))))

(event `self.OnDeployableDied`
  (`/Engine/EditorBlueprintResources/StandardMacros.Can Execute Cosmetic Events`
    (:`True`
      (`GameplayStatics.SpawnEmitterAtLocation` "/Game/Art/Effects/Particles/Explosions/P_Explosion_SonicProjector.P_Explosion_SonicProjector" (`self.K2_GetActorLocation`))
      (`GameplayStatics.PlaySoundAtLocation` "/Game/Audio/Explosions/Explosion_SonicProjector_Cue.Explosion_SonicProjector_Cue" (`self.K2_GetActorLocation`) (struct) 2.0 1.0 0.0 null null null)
      (`|ExecutionSequence`
        (:`then_0`
          (goto _label_2))
        (:`then_1`
          (bind _returnvalue (`KismetMaterialLibrary.CreateDynamicMaterialInstance` "/Game/Art/Weapons/Materials/Deployables/M_DeployableDissolve.M_DeployableDissolve" "None" "Transient"))
          (`/Engine/EditorBlueprintResources/StandardMacros.IsValid` _returnvalue
            (:`Is Valid`
              (bind _sonic_projector_core (`self.Sonic Projector Core`)
                (:`then`
                  (`PrimitiveComponent.SetMaterial` _sonic_projector_core 0 _returnvalue)
                  (`PrimitiveComponent.SetMaterial` (`self.Sonic Projector Shell1`) 0 _returnvalue)
                  (`PrimitiveComponent.SetMaterial` (`self.Sonic Projector Shell`) 0 _returnvalue)
                  (`Interpolator.InterpolateOverTimeSimple` 2.0 "EaseOut" (delegate `Death Interpolate`) (delegate `Death End`))
                  (`MaterialInstanceDynamic.SetVectorParameterValue` _returnvalue "Colour" (`KismetMathLibrary.SelectColor` (struct :`G` 0.7 :`B` 0.8 :`A` 1.0) (struct :`R` 0.83 :`G` 0.4 :`A` 1.0) (`self.bIsAlly`))))
                (:`else`)))))
        (:`then_2`
          (`|ExecutionSequence`
            (:`then_0`
              (bind _afterburner (`self.Afterburner`)
                (:`then`
                  (`ActorComponent.K2_DestroyComponent` _afterburner))
                (:`else`)))
            (:`then_1`
              (bind _afterburner1 (`self.Afterburner1`)
                (:`then`
                  (`ActorComponent.K2_DestroyComponent` _afterburner1))
                (:`else`)))
            (:`then_2`
              (bind _afterburner3 (`self.Afterburner3`)
                (:`then`
                  (`ActorComponent.K2_DestroyComponent` _afterburner3))
                (:`else`)))
            (:`then_3`
              (bind _afterburner4 (`self.Afterburner4`)
                (:`then`
                  (`ActorComponent.K2_DestroyComponent` _afterburner4))
                (:`else`)))))))))

(event `Death Interpolate`
  (params (Value :type "Float (double-precision)"))
  (`/Engine/EditorBlueprintResources/StandardMacros.IsValid` (stale `self.OnDeployableDied` _returnvalue)
    (:`Is Valid`
      (`MaterialInstanceDynamic.SetScalarParameterValue` (stale `self.OnDeployableDied` _returnvalue) "DissolveValue" (- 1.0 Value))
      (bind _pointlight (`self.PointLight`)
        (:`then`
          (`LightComponent.SetIntensity` _pointlight (`KismetMathLibrary.Lerp` 10000.0 0.0 Value)))
        (:`else`)))))

(event `Death End`
  (params (Value :type "Float (double-precision)"))
  (`SceneComponent.SetVisibility` (`self.ProjectorRoot`) false true))

(fn `UserConstructionScript`)