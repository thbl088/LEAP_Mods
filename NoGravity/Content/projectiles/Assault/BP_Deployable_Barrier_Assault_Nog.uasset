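; Deployable barrier projectile asset for the Assault Nog variant, covering only the team colouring of its shield visuals.
; On InitializeforTeam it fetches its target colour relative to player controller 0, so the tint is resolved for the local viewer.
; Scaled RGB channels of that colour drive the Color1 and Color2 material parameters on the shield and tower funnel meshes, with Color2 slightly dimmer in red.
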(event `self.InitializeForTeam`
  (params (Team :type Integer))
  (bind _sm_shieldtower_funnel (`self.SM_ShieldTower_Funnel`))
  (bind _shield (`self.shield`))
  (bind _x (.x (`KismetMathLibrary.Conv_LinearColorToVector` (`ProjectXGameState.GetTargetColour` self "None" (`GameplayStatics.GetPlayerController` 0)))))
  (bind _y (.y (`KismetMathLibrary.Conv_LinearColorToVector` (`ProjectXGameState.GetTargetColour` self "None" (`GameplayStatics.GetPlayerController` 0)))))
  (bind _z (.z (`KismetMathLibrary.Conv_LinearColorToVector` (`ProjectXGameState.GetTargetColour` self "None" (`GameplayStatics.GetPlayerController` 0)))))
  (bind _returnvalue (`KismetMathLibrary.MakeVector` (* _x 1.0) (* _y 0.25) (* _z 0.75)))
  (bind _returnvalue_2 (`KismetMathLibrary.MakeVector` (* _x 0.75) (* _y 0.25) (* _z 0.75)))
  (`MeshComponent.SetVectorParameterValueOnMaterials` _shield "Color1" _returnvalue)
  (`MeshComponent.SetVectorParameterValueOnMaterials` _shield "Color2" _returnvalue_2)
  (`MeshComponent.SetVectorParameterValueOnMaterials` _sm_shieldtower_funnel "Color1" _returnvalue)
  (`MeshComponent.SetVectorParameterValueOnMaterials` _sm_shieldtower_funnel "Color2" _returnvalue_2))

(fn `UserConstructionScript`)