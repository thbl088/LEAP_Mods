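; Assault deployable barrier: a thrown projectile that unfolds a generator into a team-coloured shield.
; The first hit starts deployment on authority; completion enables shield collision and the affliction volume.
; Cosmetic-only paths run the opening montage, interpolated material fades, impact shimmer with health-driven dissolve, and death explosion.
; Remote clients snap meshes to the stop point, and a cosmetic hit can force the opening animation if deploy state lags.
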(event `self.ReceiveBeginPlay`
  (`|ExecutionSequence`
    (:`then_0`
      (`PrimitiveComponent.SetCollisionEnabled` (`self.shieldcollision`) "NoCollision")
      (`/Engine/EditorBlueprintResources/StandardMacros.Can Execute Cosmetic Events`
        (:`True`
          (`|PlayMontage` (`self.generator`) "/Game/Art/Environment/Props/AssaultShield/Meshes/assaultshieldopen_Anim_Montage.assaultshieldopen_Anim_Montage" 1.0 0.0 "Closed"))
        (:`False`
          (`ActorComponent.SetComponentTickEnabled` (`self.generator`) false))))
    (:`then_1`
      (if (`ProjectXGameState.IsAlly` self (`GameplayStatics.GetPlayerController` 0))
        (`ActorComponent.K2_DestroyComponent` (`self.Outline`))))))

(event `self.ProjectileMovement.OnProjectileStop`
  (params (ImpactResult :type "HitResult Structure (by ref)"))
  (bind (_bblockinghit _binitialoverlap _time _distance _location) (`GameplayStatics.BreakHitResult` ImpactResult))
  (bind _outline (`self.Outline`))
  (bind _generator (`self.generator`))
  (bind _sm_shieldtower_funnel (`self.SM_ShieldTower_Funnel`))
  (`self.K2_SetActorLocation` _location false true)
  (`/Engine/EditorBlueprintResources/ActorMacros.Switch Has Authority`
    (:`Remote`
      (`SceneComponent.K2_SetWorldLocation` _generator (+ _location (`SceneComponent.RelativeLocation` _generator)) false true)
      (`SceneComponent.K2_SetWorldLocation` _sm_shieldtower_funnel (+ _location (`SceneComponent.RelativeLocation` _sm_shieldtower_funnel)) false true)
      (`SceneComponent.K2_SetWorldLocation` _outline (+ _location (`SceneComponent.RelativeLocation` _outline)) false true))))

(event `self.OnDeployComplete`
  (`PrimitiveComponent.SetCollisionEnabled` (`self.shieldcollision`) "QueryAndPhysics")
  (`ActorComponent.Activate` (`self.AfflictionVolume`) false))

(event `self.InitializeForTeam`
  (params (Team :type Integer))
  (bind _sm_shieldtower_funnel (`self.SM_ShieldTower_Funnel`))
  (bind _shield (`self.shield`))
  (bind _x (.x (`KismetMathLibrary.Conv_LinearColorToVector` (`ProjectXGameState.GetTargetColour` self "None" (`GameplayStatics.GetPlayerController` 0)))))
  (bind _y (.y (`KismetMathLibrary.Conv_LinearColorToVector` (`ProjectXGameState.GetTargetColour` self "None" (`GameplayStatics.GetPlayerController` 0)))))
  (bind _z (.z (`KismetMathLibrary.Conv_LinearColorToVector` (`ProjectXGameState.GetTargetColour` self "None" (`GameplayStatics.GetPlayerController` 0)))))
  (bind _returnvalue (`KismetMathLibrary.MakeVector` (* _x 0.5) (* _y 1.0) (* _z 0.75)))
  (bind _returnvalue_2 (`KismetMathLibrary.MakeVector` (* _x 0.25) (* _y 0.75) (* _z 0.5)))
  (`MeshComponent.SetVectorParameterValueOnMaterials` _shield "Color1" _returnvalue)
  (`MeshComponent.SetVectorParameterValueOnMaterials` _shield "Color2" _returnvalue_2)
  (`MeshComponent.SetVectorParameterValueOnMaterials` _sm_shieldtower_funnel "Color1" _returnvalue)
  (`MeshComponent.SetVectorParameterValueOnMaterials` _sm_shieldtower_funnel "Color2" _returnvalue_2))

(event `self.OnDeployableDied`
  (bind _audiocomponent (`self.AudioComponent`))
  (bind _returnvalue (`SceneComponent.K2_GetComponentLocation` (`self.generator`)))
  (`ActorComponent.Deactivate` (`self.AfflictionVolume`))
  (`/Engine/EditorBlueprintResources/StandardMacros.Can Execute Cosmetic Events`
    (:`True`
      (`Interpolator.InterpolateOverTimeSimple` 1.0 "ExpoOut" (delegate `FadeOut`))
      (`PrimitiveComponent.SetCollisionEnabled` (`self.shieldcollision`) "NoCollision")
      (`GameplayStatics.SpawnEmitterAtLocation` "/Game/Art/Effects/Particles/Explosions/P_Explosion_VehicleDeath_Bike.P_Explosion_VehicleDeath_Bike" _returnvalue)
      (`GameplayStatics.PlaySoundAtLocation` "/Game/Audio/Explosions/Explosion_Rocket_Cue.Explosion_Rocket_Cue" _returnvalue (struct) 1.0 1.0 0.0 null null null)
      (`/Engine/EditorBlueprintResources/StandardMacros.IsValid` _audiocomponent
        (:`Is Valid`
          (`AudioComponent.FadeOut` _audiocomponent 0.5 0.0 "Linear"))))))

(event `FadeOut`
  (params (Value :type "Float (double-precision)"))
  (bind _shield (`self.shield`))
  (`MeshComponent.SetScalarParameterValueOnMaterials` _shield "DissolveValue" (`KismetMathLibrary.Lerp` 1.0 0.0 Value))
  (`MeshComponent.SetScalarParameterValueOnMaterials` (`self.SM_ShieldTower_Funnel`) "DissolveValue" (`KismetMathLibrary.Lerp` 1.0 0.0 Value))
  (`MeshComponent.SetScalarParameterValueOnMaterials` _shield "OpacityPower" (`KismetMathLibrary.Lerp` 50.0 0.0 Value))
  (`MeshComponent.SetScalarParameterValueOnMaterials` (`self.SM_ShieldTower_Funnel`) "OpacityPower" (`KismetMathLibrary.Lerp` 50.0 0.0 Value))
  (`MeshComponent.SetScalarParameterValueOnMaterials` (`self.shield`) "NormalOffset" (`KismetMathLibrary.Lerp` 30.0 1000.0 Value)))

(event `self.OnDeployStart`
  (bind _returnvalue (/ (`self.DeployTime`) 2.0))
  (`/Engine/EditorBlueprintResources/StandardMacros.Can Execute Cosmetic Events` :!label _label
    (:`True`
      (`/Engine/EditorBlueprintResources/StandardMacros.DoOnce` false
        (:`Completed`
          (`|ExecutionSequence`
            (:`then_0`
              (`|PlayMontage` (`self.generator`) "/Game/Art/Environment/Props/AssaultShield/Meshes/assaultshieldopen_Anim_Montage.assaultshieldopen_Anim_Montage" 1.0 0.0 "Default"
                (:`then`
                  (`GameplayStatics.PlaySoundAtLocation` "/Game/Audio/Weapons/AssaultShield/shieldopen_Cue.shieldopen_Cue" (`self.K2_GetActorLocation`) (struct) 1.0 1.0 0.0 null null null))))
            (:`then_1`
              (`KismetSystemLibrary.Delay` _returnvalue)
              (`Interpolator.InterpolateOverTime` 0.0 _returnvalue 0.0 1.0 "EaseIn" (delegate `FadeIn`))
              (`GameplayStatics.SpawnEmitterAtLocation` "/Game/ThirdPartyAssets/FXVarietyPack/Particles/P_ky_hit1.P_ky_hit1" (`SceneComponent.K2_GetComponentLocation` (`self.generator`)) (struct) (10.0 10.0 10.0))
              (bind _returnvalue_2 (`GameplayStatics.SpawnSoundAtLocation` "/Game/Audio/Weapons/AssaultShield/shieldburst_Cue.shieldburst_Cue" (`self.K2_GetActorLocation`) (struct) 1.0 1.0 0.0 null null))
              (set `self.AudioComponent` _returnvalue_2)
              (`GameplayStatics.PlaySoundAtLocation` "/Game/Audio/Weapons/AssaultShield/shieldopen_Cue1.shieldopen_Cue1" (`self.K2_GetActorLocation`) (struct) 1.0 1.0 0.0 null null null))))))))

(event `ForceAnim`
  (goto _label))

(event `FadeIn`
  (params (Value :type "Float (double-precision)"))
  (bind _shield (`self.shield`))
  (`MeshComponent.SetScalarParameterValueOnMaterials` _shield "DissolveValue" Value)
  (`MeshComponent.SetScalarParameterValueOnMaterials` (`self.SM_ShieldTower_Funnel`) "DissolveValue" Value)
  (`MeshComponent.SetScalarParameterValueOnMaterials` _shield "OpacityPower" (`KismetMathLibrary.Lerp` 0.0 50.0 Value))
  (`MeshComponent.SetScalarParameterValueOnMaterials` (`self.SM_ShieldTower_Funnel`) "OpacityPower" (`KismetMathLibrary.Lerp` 0.0 50.0 Value))
  (`MeshComponent.SetScalarParameterValueOnMaterials` (`self.shield`) "NormalOffset" (`KismetMathLibrary.Lerp` -1000.0 30.0 Value))
  (`/Engine/EditorBlueprintResources/StandardMacros.DoOnce` false
    (:`Completed`
      (`SceneComponent.SetHiddenInGame` (`self.shield`) false false)
      (`SceneComponent.SetHiddenInGame` (`self.SM_ShieldTower_Funnel`) false false))))

(event `self.ReceiveHit`
  (params (MyComp :type "PrimitiveComponent Object Reference") (Other :type "Actor Object Reference") (OtherComp :type "PrimitiveComponent Object Reference") (bSelfMoved :type Boolean) (HitLocation :type "Vector Structure") (HitNormal :type "Vector Structure") (NormalImpulse :type "Vector Structure") (Hit :type "HitResult Structure (by ref)"))
  (bind _returnvalue (`self.GetDeployableState`))
  (bind _returnvalue_2 (/ (`HealthInterface.GetHealth`) (`HealthInterface.GetMaxHealth`)))
  (`|ExecutionSequence`
    (:`then_0`
      (if (!= MyComp (`self.Sphere`))
        (`/Engine/EditorBlueprintResources/StandardMacros.Can Execute Cosmetic Events`
          (:`True`
            (`Interpolator.ClearInterpolation` self (`self.ShimmerInterpID`))
            (`MeshComponent.SetVectorParameterValueOnMaterials` (`self.shield`) "HitPosition" HitLocation)
            (bind _returnvalue_3 (`Interpolator.InterpolateOverTimeSimple` 0.5 "ExpoOut" (delegate `Shimmer`)))
            (set `self.ShimmerInterpID` _returnvalue_3)
            (`MeshComponent.SetScalarParameterValueOnMaterials` (`self.shield`) "DissolveValue" (`KismetMathLibrary.Lerp` 0.3 1.0 _returnvalue_2))
            (`MeshComponent.SetScalarParameterValueOnMaterials` (`self.shield`) "DissolveEdgeWidth" (`KismetMathLibrary.Lerp` 6.0 1.75 (`KismetMathLibrary.FClamp` (+ _returnvalue_2 0.5))))
            (`GameplayStatics.PlaySoundAtLocation` "/Game/Audio/Deployables/Containers/ContainerImpactSmall_Cue.ContainerImpactSmall_Cue" (`self.K2_GetActorLocation`) (struct) 1.0 1.0 0.0 null null null)
            (`/Engine/EditorBlueprintResources/StandardMacros.DoOnce` false
              (:`Completed`
                (if (and (`|EnumInequality` _returnvalue "StartingUp") (`|EnumInequality` _returnvalue "Activated"))
                  (`self.ForceAnim`))))))))
    (:`then_1`
      (`/Engine/EditorBlueprintResources/ActorMacros.Switch Has Authority`
        (:`Authority`
          (`/Engine/EditorBlueprintResources/StandardMacros.DoOnce` false
            (:`Completed`
              (`self.DeployStart` true))))))
    (:`then_2`
      (`/Engine/EditorBlueprintResources/StandardMacros.Can Execute Cosmetic Events`
        (:`True`
          (if (== MyComp (`self.Sphere`))
            (`GameplayStatics.SpawnEmitterAtLocation` "/Game/Art/Effects/Particles/BulletImpacts/Deprecated/PS_Impact_Dirt_Large.PS_Impact_Dirt_Large" (`SceneComponent.K2_GetComponentLocation` (`self.Sphere`)))))))))

(event `Shimmer`
  (params (Value :type "Float (double-precision)"))
  (`MeshComponent.SetScalarParameterValueOnMaterials` (`self.shield`) "HitRadius" (`KismetMathLibrary.Lerp` 0.0 500.0 Value))
  (`MeshComponent.SetScalarParameterValueOnMaterials` (`self.shield`) "HitHardness" (`KismetMathLibrary.Lerp` 0.5 1.0 Value))
  (`MeshComponent.SetScalarParameterValueOnMaterials` (`self.shield`) "HitVisibility" (`KismetMathLibrary.Lerp` 1.0 0.0 Value)))

(event `self.OnDeployDeactivated`
  (`/Engine/EditorBlueprintResources/ActorMacros.Switch Has Authority`
    (:`Authority`
      (`self.ClearDeployable`))))

(fn `UserConstructionScript`)