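; Juggernaut variant of the ProjectX character that reflects damage back at non-allied attackers.
; When it takes damage, it applies the same amount to the damage causer, credited to the victim and its instigator controller.
; On death, it retaliates with a large fixed hit against the killer.
; Both events first compare the causer's team with the victim, so allies are never hit back.
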(event `self.DamageTaken`
  (params (Victim :type "Actor Object Reference") (Damage :type "Float (single-precision)") (DamageEvent :type "DamageEvent Structure (by ref)") (EventInstigator :type "Controller Object Reference") (DamageCauser :type "Actor Object Reference") (InstigatorPlayerState :type "PlayerState Object Reference"))
  (bind _returnvalue (message `TeamInterface.GetTeam` DamageCauser))
  (if (not (`ProjectXGameState.IsAllyByTeam` _returnvalue Victim))
    (`GameplayStatics.ApplyDamage` DamageCauser Damage (`self.GetInstigatorController` Victim) Victim)))

(event `self.Died`
  (params (Victim :type "Actor Object Reference") (Damage :type "Float (single-precision)") (DamageEvent :type "DamageEvent Structure (by ref)") (EventInstigator :type "Controller Object Reference") (DamageCauser :type "Actor Object Reference") (InstigatorPlayerState :type "PlayerState Object Reference"))
  (bind _returnvalue (message `TeamInterface.GetTeam` DamageCauser))
  (if (not (`ProjectXGameState.IsAllyByTeam` _returnvalue Victim))
    (`GameplayStatics.ApplyDamage` DamageCauser 1000.0 (`self.GetInstigatorController` Victim) Victim)))

(fn `UserConstructionScript`
  (`parent.UserConstructionScript`))