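; Character Blueprint for a Fiesta variant of the ProjectX character, giving it a randomized loadout on spawn.
; BeginPlay draws from class arrays to fill two weapon, primary, secondary, ultimate and vehicle ability slots through the weapon component, spacing adds with Delays.
; Parent BeginPlay runs only after the final add.
; A RandomBuild macro duplicates the sequence but fixes the secondary ability to index 1, and is not called here.
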(event `self.ReceiveBeginPlay`
  (bind _returnvalue (`self.GetWeaponComponent`))
  (bind _duration (`self.Duration`))
  (`KismetSystemLibrary.Delay` 0.2)
  (`WeaponComponent.AddWeapon` _returnvalue (`KismetArrayLibrary.Array_Random` (`self.Weapons`)) "PrimaryWeapon" false)
  (`KismetSystemLibrary.Delay` _duration)
  (`WeaponComponent.AddWeapon` _returnvalue (`KismetArrayLibrary.Array_Random` (`self.Weapons`)) "SecondaryWeapon" false)
  (`KismetSystemLibrary.Delay` _duration)
  (`WeaponComponent.AddWeapon` _returnvalue (`KismetArrayLibrary.Array_Random` (`self.PrimaryAbility`)) "PrimaryAbility" false)
  (`KismetSystemLibrary.Delay` _duration)
  (`WeaponComponent.AddWeapon` _returnvalue (`KismetArrayLibrary.Array_Random` (`self.SecondaryAbility`)) "SecondaryAbility" false)
  (`KismetSystemLibrary.Delay` _duration)
  (`WeaponComponent.AddWeapon` _returnvalue (`KismetArrayLibrary.Array_Random` (`self.Ult`)) "UltimateAbility" false)
  (`KismetSystemLibrary.Delay` _duration)
  (`WeaponComponent.AddWeapon` _returnvalue (`KismetArrayLibrary.Array_Random` (`self.PV`)) "VehicleAbility" false)
  (`parent.ReceiveBeginPlay`))

(fn `UserConstructionScript`
  (`parent.UserConstructionScript`))