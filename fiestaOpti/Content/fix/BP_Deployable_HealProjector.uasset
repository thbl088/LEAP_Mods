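; Thrown deployable heal projector that lands and projects a healing area through an affliction volume.
; On projectile stop, the authority starts deployment while cosmetic-capable instances play impact effects and the deploy montage.
; Completion or reactivation enables the heal volume and fades in a funnel and sphere, tinted by viewer-relative healing colour.
; Deactivation stops healing and reverses the montage; deactivation and death both fade out visuals and loop audio.
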(event `self.ReceiveBeginPlay`
  (`PrimitiveComponent.SetCollisionEnabled` (`self.SkeletalMesh`) "NoCollision")
  (`/Engine/EditorBlueprintResources/StandardMacros.Can Execute Cosmetic Events`
    (:`True`
      (`SceneComponent.SetHiddenInGame` (`self.Sphere`) true true)
      (bind _returnvalue (`GameplayStatics.SpawnSoundAttached` "/Game/Audio/Abilities/Stasis/Stasis_Cue_Heal.Stasis_Cue_Heal" (`self.SphereRoot`) "None" (0.0 0.0 0.0) (struct) "KeepRelativeOffset" false 1.0 1.0 0.0 null null))
      (set `self.ProjectileSound` _returnvalue))
    (:`False`
      (`SkeletalMeshComponent.SetAnimInstanceClass` (`self.SkeletalMesh`) null)
      (`ActorComponent.K2_DestroyComponent` (`self.Sphere`))
      (`ActorComponent.K2_DestroyComponent` (`self.Funnel`))
      (`ActorComponent.K2_DestroyComponent` (`self.Outline`)))))

(event `self.ProjectileMovement.OnProjectileStop`
  (params (ImpactResult :type "HitResult Structure (by ref)"))
  (bind _returnvalue (`self.K2_GetActorLocation`))
  (`|ExecutionSequence`
    (:`then_0`
      (`/Engine/EditorBlueprintResources/ActorMacros.Switch Has Authority`
        (:`Authority`
          (`self.K2_SetActorLocation` (`.Location` (`GameplayStatics.BreakHitResult` ImpactResult)))
          (`self.DeployStart` false))))
    (:`then_1`
      (`/Engine/EditorBlueprintResources/StandardMacros.Can Execute Cosmetic Events`
        (:`True`
          (`AudioComponent.Stop` (`self.ProjectileSound`))
          (`GameplayStatics.PlaySoundAtLocation` "/Game/Audio/Deployables/Containers/ContainerImpact_Cue.ContainerImpact_Cue" _returnvalue (struct) 1.0 1.0 0.0 null null null)
          (`GameplayStatics.PlayWorldCameraShake` "/Game/Blueprints/Weapons/Deployable/Deployables/Containers/BP_ContainerLandShake.BP_ContainerLandShake_C" _returnvalue 1000.0 5000.0)
          (`GameplayStatics.SpawnEmitterAtLocation` "/Game/Art/Effects/Particles/BulletImpacts/Deprecated/PS_Impact_Deployable.PS_Impact_Deployable" _returnvalue)
          (`AdvancedWidgetComponent.CreateWidgetComponent` self (`KismetMathLibrary.MakeTransform` (0.0 0.0 300.0)) "/Game/Blueprints/UI/World/BP_DeployabeHudInfoWidgetComponent.BP_DeployabeHudInfoWidgetComponent_C")
          (`|PlayMontage` (`self.SkeletalMesh`) "/Game/Art/Items/Animations/ANM_HealthGenerator_Deploy.ANM_HealthGenerator_Deploy"
            (:`then`
              (bind _returnvalue_2 (`GameplayStatics.SpawnEmitterAttached` "/Game/Art/Effects/Particles/Trails/PS_DeployableTrail.PS_DeployableTrail" (`self.RootComponent`)))
              (bind _output_get (set `self.DeployTrail` _returnvalue_2))
              (`KismetSystemLibrary.Delay` 0.1)
              (`ActorComponent.Deactivate` _output_get))))))))

(event `self.OnDeployStart`
  (`PrimitiveComponent.SetCollisionEnabled` (`self.SkeletalMesh`) "QueryAndPhysics"))

(event `self.OnDeployReActivated`
  (bind _returnvalue (`SceneComponent.K2_GetComponentLocation` (`self.Funnel`)))
  (`|ExecutionSequence`
    (:`then_0`
      (goto _label_2 :!via `Reset`))
    (:`then_1`
      (set `self.Deactivated` false)
      (if (not (`self.Deactivated`)) :!label _label
        (`/Engine/EditorBlueprintResources/StandardMacros.DoOnce` false :!label _label_2
          (:`Completed`
            (`|ExecutionSequence`
              (:`then_0`
                (`/Engine/EditorBlueprintResources/StandardMacros.Can Execute Cosmetic Events`
                  (:`True`
                    (bind _generatorloop (`self.GeneratorLoop`)
                      (:`then`
                        (`AudioComponent.Play` _generatorloop 0.0))
                      (:`else`
                        (bind _returnvalue_2 (`GameplayStatics.SpawnSoundAtLocation` "/Game/Audio/Weapons/HealProjector/loop_Cue.loop_Cue" (`self.K2_GetActorLocation`) (struct) 1.0 1.0 0.0 null null))
                        (set `self.GeneratorLoop` _returnvalue_2)))
                    (`SceneComponent.SetHiddenInGame` (`self.Sphere`) false true)
                    (`Interpolator.InterpolateOverTime` 0.0 1.0 0.0 1.0 "EaseOut" (delegate `Interp`) (delegate `FunnelActive`))
                    (`MeshComponent.SetScalarParameterValueOnMaterials` (`self.Sphere`) "OverallOpacity" 0.0)
                    (`MeshComponent.SetScalarParameterValueOnMaterials` (`self.Funnel`) "OverallOpacity" 0.0)
                    (`GameplayStatics.SpawnEmitterAtLocation` "/Game/ThirdPartyAssets/FireEnergyVFX/Particles/P_Appear1.P_Appear1" _returnvalue)
                    (`GameplayStatics.PlaySoundAtLocation` "/Game/Audio/Weapons/HealProjector/emit_Cue.emit_Cue" _returnvalue (struct) 1.0 1.0 0.0 null null null)
                    (bind _loopingparticlesystem (`self.LoopingParticleSystem`)
                      (:`then`
                        (`ActorComponent.Activate` _loopingparticlesystem false))
                      (:`else`
                        (bind _returnvalue_3 (`GameplayStatics.SpawnEmitterAtLocation` "/Game/ThirdPartyAssets/FireEnergyVFX/Particles/P_Portal1.P_Portal1" _returnvalue))
                        (set `self.LoopingParticleSystem` _returnvalue_3))))))
              (:`then_1`
                (`ActorComponent.Activate` (`self.AfflictionVolumeHeal`) false)))))))))

(event `Interp`
  (params (Value :type "Float (double-precision)"))
  (`MeshComponent.SetScalarParameterValueOnMaterials` (`self.Funnel`) "OverallOpacity" Value))

(event `self.OnDeployComplete`
  (goto _label))

(event `FadeSphere`
  (params (Value :type "Float (double-precision)"))
  (`MeshComponent.SetScalarParameterValueOnMaterials` (`self.Sphere`) "OverallOpacity" Value))

(event `FunnelActive`
  (params (Value :type "Float (double-precision)"))
  (`Interpolator.InterpolateOverTime` 0.0 1.0 0.0 3.0 "EaseInOut" (delegate `FadeSphere`)))

(event `self.InitializeForTeam`
  (params (Team :type Integer))
  (bind _funnel (`self.Funnel`))
  (bind _sphere (`self.Sphere`))
  (bind _returnvalue (`KismetMathLibrary.Conv_LinearColorToVector` (`ProjectXGameState.GetTargetColour` self "Healing" (`GameplayStatics.GetPlayerController` 0))))
  (set `self.Team` Team)
  (`|ExecutionSequence`
    (:`then_0`
      (`/Engine/EditorBlueprintResources/StandardMacros.IsValid` _funnel
        (:`Is Valid`
          (`MeshComponent.SetVectorParameterValueOnMaterials` (`self.SkeletalMesh`) "Colour" _returnvalue)
          (`MeshComponent.SetVectorParameterValueOnMaterials` _funnel "Colour" _returnvalue)
          (`MeshComponent.SetVectorParameterValueOnMaterials` _funnel "ShieldHoleColour" _returnvalue)
          (`MeshComponent.SetVectorParameterValueOnMaterials` _funnel "ShieldIntersectColor" _returnvalue))))
    (:`then_1`
      (`/Engine/EditorBlueprintResources/StandardMacros.IsValid` _sphere
        (:`Is Valid`
          (`MeshComponent.SetVectorParameterValueOnMaterials` _sphere "MainColor" (* _returnvalue 10.0))
          (`MeshComponent.SetVectorParameterValueOnMaterials` _sphere "EmissiveLineColor" (* _returnvalue 50.0))
          (`MeshComponent.SetVectorParameterValueOnMaterials` _sphere "DepthFadeColour" (* _returnvalue 0.2)))))))

(event `self.OnDeployDeactivated`
  (bind _loopingparticlesystem (`self.LoopingParticleSystem`))
  (`|ExecutionSequence`
    (:`then_0`
      (`/Engine/EditorBlueprintResources/ActorMacros.Switch Has Authority`
        (:`Authority`
          (`ActorComponent.Deactivate` (`self.AfflictionVolumeHeal`)))))
    (:`then_1`
      (`/Engine/EditorBlueprintResources/StandardMacros.Can Execute Cosmetic Events`
        (:`True`
          (`|PlayMontage` (`self.SkeletalMesh`) "/Game/Art/Items/Animations/ANM_HealthGenerator_Deploy.ANM_HealthGenerator_Deploy" -1.0
            (:`then`
              (set `self.Deactivated` true :!label _label_3)
              (bind _generatorloop (`self.GeneratorLoop`)
                (:`then`
                  (`AudioComponent.FadeOut` _generatorloop 0.5 0.0 "Linear"))
                (:`else`
                  _))
              (`Interpolator.InterpolateOverTime` 0.0 1.0 1.0 0.0 "EaseOut" (delegate `InterpOut`) (delegate `End`))
              (`/Engine/EditorBlueprintResources/StandardMacros.IsValid` _loopingparticlesystem
                (:`Is Valid`
                  (`ActorComponent.Deactivate` _loopingparticlesystem))))))))))

(event `self.OnDeployableDied`
  (`/Engine/EditorBlueprintResources/StandardMacros.Can Execute Cosmetic Events`
    (:`True`
      (`GameplayStatics.SpawnEmitterAtLocation` "/Game/Art/Effects/Particles/Explosions/P_Explosion_VehicleDeath_Bike.P_Explosion_VehicleDeath_Bike" (`self.K2_GetActorLocation`))
      (`GameplayStatics.PlaySoundAtLocation` "/Game/Audio/EnvironmentTraps/Meteor/MeteorExplosion_Cue.MeteorExplosion_Cue" (`self.K2_GetActorLocation`) (struct) 1.0 1.0 0.0 null null null)
      (`SceneComponent.SetVisibility` (`self.SkeletalMesh`) false false)
      (goto _label_3))))

(event `InterpOut`
  (params (Value :type "Float (double-precision)"))
  (`|ExecutionSequence`
    (:`then_0`
      (bind _funnel (`self.Funnel`)
        (:`then`
          _)
        (:`else`)))
    (:`then_1`
      (bind _sphere (`self.Sphere`)
        (:`then`
          _)
        (:`else`))))
  (`MeshComponent.SetScalarParameterValueOnMaterials` _funnel "OverallOpacity" Value)
  (`MeshComponent.SetScalarParameterValueOnMaterials` _sphere "OverallOpacity" Value))

(event `End`
  (params (Value :type "Float (double-precision)"))
  (bind _sphere (`self.Sphere`)
    (:`then`
      (`SceneComponent.SetHiddenInGame` _sphere true true))
    (:`else`)))

(fn `UserConstructionScript`)