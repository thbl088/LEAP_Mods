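; BP_DamagingAffliction_HealBeam is a damaging affliction that supplies screen and audio feedback for the damage side of the heal beam.
; On start it adds the W_HealProjectorOverlay_Damage widget to the viewport, only when the owning character is locally controlled, and removes it on end.
; Each damage event plays a negative-hit beam sound attached to the owning character's mesh.
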(event `self.K2_Start`
  (bind _returnvalue (`self.GetOwningCharacter`))
  (`parent.K2_Start`)
  (`/Engine/EditorBlueprintResources/StandardMacros.IsValid` _returnvalue
    (:`Is Valid`
      (if (`Pawn.IsLocallyControlled` _returnvalue)
        (`self.Widget`
          (:`then`)
          (:`else`
            (bind _returnvalue_2 (`|CreateWidget` "/Game/Blueprints/UI/W_HealProjectorOverlay_Damage.W_HealProjectorOverlay_Damage_C" (`GameplayStatics.GetPlayerController` 0)))
            (bind _output_get (set `self.Widget` _returnvalue_2))
            (`UserWidget.AddToViewport` _output_get 0)))))))

(event `self.K2_End`
  (`parent.K2_End`)
  (bind _widget (`self.Widget`)
    (:`then`
      (`Widget.RemoveFromParent` _widget))
    (:`else`)))

(event `self.On Damage Done`
  (`GameplayStatics.SpawnSoundAttached` "/Game/Audio/Weapons/RepairGun/Damage_Beam_Negative_Hit.Damage_Beam_Negative_Hit" (`Character.Mesh` (`self.GetOwningCharacter`)) "None" (0.0 0.0 0.0) (struct) "KeepRelativeOffset" false 1.0 1.0 0.0 null null))