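; BP_FlagCapture is a Capture the Flag team point that homes a flag and reacts to captures.
; On begin play it waits for the local player state, tints its base by team relative to that player on team changes, and adds a cosmetic icon widget.
; Flag reset moves the flag back to FlagPoint.
; Capture spawns a particle effect, and the authority broadcasts a team-tagged server message.
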(event `self.ReceiveBeginPlay`
  (`|ExecutionSequence`
    (:`then_0`
      (bind _playerstate (`BlueprintAsyncActionGetPlayerState.AsyncGetPlayerState` (`GameplayStatics.GetPlayerController` 0))
        (:`OnPlayerStateAcquired`
          (bind _asproject_xplayer_state (cast `ProjectXPlayerState` _playerstate))
          (add `ProjectXPlayerState.OnPlayerChangedTeam` _asproject_xplayer_state (delegate `OnTeamChanged`))
          (`self.OnTeamChanged` null))))
    (:`then_1`
      (`/Engine/EditorBlueprintResources/StandardMacros.Can Execute Cosmetic Events`
        (:`True`
          (`AdvancedWidgetComponent.CreateWidgetComponent` self (`self.RelativeIconLocation`) "/Game/Blueprints/UI/GameModes/CaptureTheFlag/BP_FlagSpawnWidgetComponent.BP_FlagSpawnWidgetComponent_C"))))))

(event `OnTeamChanged`
  (params (PlayerState :type "ProjectXPlayerState Object Reference") (Team :type Byte))
  (`MeshComponent.SetVectorParameterValueOnMaterials` (`self.Base`) "TeamColour" (`KismetMathLibrary.Conv_LinearColorToVector` (`ProjectXGameState.GetTargetColourByTeam` (`TeamInterface.GetTeam`) "TeamColour1" (`GameplayStatics.GetPlayerController` 0)))))

(event `self.OnFlagReset`
  (bind _returnvalue (`self.GetFlag`))
  (`self.K2_SetActorLocation` _returnvalue (`SceneComponent.K2_GetComponentLocation` (`self.FlagPoint`)) false false)
  (`self.K2_SetActorRotation` _returnvalue (`SceneComponent.K2_GetComponentRotation` (`self.FlagPoint`)) false))

(event `self.OnFlagCaptured`
  (`GameplayStatics.SpawnEmitterAtLocation` "/Game/Art/Effects/Particles/Goals/PS_CaptureTheFlag.PS_CaptureTheFlag" (`self.K2_GetActorLocation`))
  (`/Engine/EditorBlueprintResources/ActorMacros.Switch Has Authority`
    (:`Authority`
      (`BroadcastMessage.BroadcastServerMessage` "/Game/Blueprints/BroadcastMessage/Gamemodes/CaptureTheFlag/BP_BroadcastMessage_CTF_FlagCaptured.BP_BroadcastMessage_CTF_FlagCaptured_C" (`TeamInterface.GetTeam`)))))

(fn `UserConstructionScript`)