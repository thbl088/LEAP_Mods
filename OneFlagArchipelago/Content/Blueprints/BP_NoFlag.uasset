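; BP_NoFlag is a Capture the Flag flag actor that reacts to home, carried and dropped states.
; State updates print the state and keep capsule collision off, enabling damped physics only when dropped.
; Cosmetic-only branches hide the flag while carried, broadcast taken and dropped messages with its team, and show the home widget on BeginPlay.
; The pickup update checks eligibility but does nothing with it.
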(event `self.ReceiveBeginPlay`
  (`/Engine/EditorBlueprintResources/StandardMacros.Can Execute Cosmetic Events`
    (:`True`
      (`/Engine/EditorBlueprintResources/StandardMacros.IsValid` (`self.BP_FlagWidgetComponent`)
        (:`Is Valid`
          (set `/Game/Blueprints/UI/GameModes/CaptureTheFlag/BP_FlagWidgetComponent.Visiblity at Home` "SelfHitTestInvisible" (`self.BP_FlagWidgetComponent`)))))))

(event `self.FlagStatUpdated`
  (bind _returnvalue (`self.GetCapsuleComponent`))
  (bind _returnvalue_2 (`self.GetCapsuleComponent`))
  (bind _returnvalue_3 (`self.GetCapsuleComponent`))
  (bind _flagstate (break `FlagInfo` (`self.GetFlagInfo`)))
  (`KismetSystemLibrary.PrintString` (`|GetEnumeratorNameAsString` _flagstate))
  (switch `EFlagState` _flagstate
    (:`HOME`
      (`PrimitiveComponent.SetCollisionEnabled` _returnvalue "NoCollision")
      (`PrimitiveComponent.SetSimulatePhysics` _returnvalue false)
      (`/Engine/EditorBlueprintResources/StandardMacros.Can Execute Cosmetic Events`
        (:`True`
          (`self.SetActorHiddenInGame` false))))
    (:`CARRIED`
      (`PrimitiveComponent.SetCollisionEnabled` _returnvalue_3 "NoCollision")
      (`PrimitiveComponent.SetSimulatePhysics` _returnvalue_3 false)
      (`/Engine/EditorBlueprintResources/StandardMacros.Can Execute Cosmetic Events`
        (:`True`
          (`self.SetActorHiddenInGame` true)
          (`BroadcastMessage.BroadcastServerMessage` "/Game/Blueprints/BroadcastMessage/Gamemodes/CaptureTheFlag/BP_BroadcastMessage_CTF_FlagTaken.BP_BroadcastMessage_CTF_FlagTaken_C" (`TeamInterface.GetTeam`)))))
    (:`DROPPED`
      (`PrimitiveComponent.SetCollisionEnabled` _returnvalue_2 "NoCollision")
      (`PrimitiveComponent.SetSimulatePhysics` _returnvalue_2 true)
      (`PrimitiveComponent.SetLinearDamping` _returnvalue_2 0.5)
      (`/Engine/EditorBlueprintResources/StandardMacros.Can Execute Cosmetic Events`
        (:`True`
          (`self.SetActorHiddenInGame` false)
          (`BroadcastMessage.BroadcastServerMessage` "/Game/Blueprints/BroadcastMessage/Gamemodes/CaptureTheFlag/BP_BroadcastMessage_CTF_FlagDropped.BP_BroadcastMessage_CTF_FlagDropped_C" (`TeamInterface.GetTeam`)))))))

(event `self.FlagPickupUpdated`
  (if (`self.CanBePickedUp`)
    _))

(fn `UserConstructionScript`)