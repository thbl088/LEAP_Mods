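; Explosion actor for the pull grenade that yanks nearby characters toward its center when it detonates.
; While a delayed explosion counts down, an audio component's pitch ramps up, the sphere's emissive flickers more intensely, and a warning widget is initialized for the team.
; On trigger it plays sound, particles and camera shake, applies inward velocity impulses via PullArea, then destroys itself, all behind the cosmetic-events check.
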(event `self.OnExplosionTriggered`
  (bind _returnvalue (`self.K2_GetActorLocation`))
  (`/Engine/EditorBlueprintResources/StandardMacros.Can Execute Cosmetic Events`
    (:`True`
      (`GameplayStatics.PlaySoundAtLocation` "/Game/Audio/Explosions/Explosion_StickyGrenade.Explosion_StickyGrenade" _returnvalue (struct) 0.9 1.0 0.0 null null null)
      (`GameplayStatics.SpawnEmitterAtLocation` "/Game/Art/Effects/Particles/Explosions/P_Explosion_StickyGrenade.P_Explosion_StickyGrenade" _returnvalue)
      (`GameplayStatics.PlayWorldCameraShake` "/Game/ThirdPartyAssets/IBFPSStarterPack/Blueprints/BP_BlastShake.BP_BlastShake_C" (`self.K2_GetActorLocation`) 3000.0 10000.0)
      (`self.PullArea`)
      (`self.K2_DestroyActor`))))

(event `self.ReceiveBeginPlay`
  (`parent.ReceiveBeginPlay`)
  (`|ExecutionSequence`
    (:`then_0`
      (`/Engine/EditorBlueprintResources/StandardMacros.Can Execute Cosmetic Events`
        (:`True`
          (if (`self.bDelayExplosion`)
            (`KismetSystemLibrary.Delay` 0.2)
            (`Interpolator.InterpolateOverTimeSimple` (`self.ExplosionDelay`) "Linear" (delegate `On Warning Updates`))
            (bind _returnvalue (`AddComponent|NODE_AddAudioComponent-0`))))))
    (:`then_1`
      (bind _bp_projectilewarningwidgetcomponent (`self.BP_ProjectileWarningWidgetComponent`)
        (:`then`
          (`/Game/Blueprints/UI/Weapons/BP_GrenadeWarningWidgetComponent.InitializeForTeam` _bp_projectilewarningwidgetcomponent (`TeamInterface.GetTeam`)))
        (:`else`)))))

(event `On Warning Updates`
  (params (Value :type "Float (double-precision)"))
  (`/Engine/EditorBlueprintResources/StandardMacros.IsValid` (stale `self.ReceiveBeginPlay` _returnvalue)
    (:`Is Valid`
      (`AudioComponent.SetFloatParameter` (stale `self.ReceiveBeginPlay` _returnvalue) "PitchControl" (* Value 2.0)))))

(event `self.ReceiveTick`
  (params (DeltaSeconds :type "Float (single-precision)"))
  (set `self.Time` (+ DeltaSeconds (`self.Time`)))
  (`MeshComponent.SetScalarParameterValueOnMaterials` (`self.Sphere1`) "EmissiveMultiplier" (`KismetMathLibrary.RandomFloatInRange` 1.0 (+ (* (`KismetMathLibrary.FClamp` (- 1.0 (- (`self.ExplosionDelay`) (`self.Time`)))) 10.0) 1.0))))

(fn `PullArea`
  (for _array_element (`ProjectXGameplayStatics.GetTargetsInRadius` (`self.K2_GetActorLocation` self) (`self.RadiusBump`))
    (bind _asbp_project_xcharacter (cast `/Game/Blueprints/Gameplay/PlayerClasses/BP_ProjectXCharacter` _array_element))
    (`CharacterMovementComponent.AddImpulse` (`Character.CharacterMovement` _asbp_project_xcharacter) (* (`KismetMathLibrary.Normal` (- (`self.K2_GetActorLocation` self) (`self.K2_GetActorLocation` _asbp_project_xcharacter))) (`self.StrengthBump`)) true)))

(fn `UserConstructionScript`)