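; Game mode for an Infected match, where one random player starts on the infected team and the rest start as hunted.
; Login and logout asynchronously acquire player states to maintain a player list, exposed with the default team through GetPlayerList.
; When the match enters In Progress, it assigns teams through SetTeam messages.
; Each new player's death event is bound on login, but the handler only prints a debug string.
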(event `self.K2_PostLogin`
  (params (NewPlayer :type "PlayerController Object Reference"))
  ;[1 1 1] Login
  (message `HealthInterface.BindToDeathEvent` NewPlayer (delegate `OnDeath`))
  (bind _playerstate (`BlueprintAsyncActionGetPlayerState.AsyncGetPlayerState` NewPlayer)
    (:`OnPlayerStateAcquired`
      ;;[1 1 1] We add a new player to the player list
      (`KismetArrayLibrary.Array_Insert` (`self.PlayerStateList`) _playerstate))))

(event `OnDeath`
  (params (Victim :type "Actor Object Reference") (Damage :type "Float (double-precision)") (DamageEvent :type "DamageEvent Structure (by ref)") (EventInstigator :type "Controller Object Reference") (DamageCauser :type "Actor Object Reference") (InstigatorPlayerState :type "PlayerState Object Reference"))
  ;[1 1 1] Login
  (`KismetSystemLibrary.PrintString` "Hello"))

(event `self.K2_OnLogout`
  (params (ExitingController :type "Controller Object Reference"))
  ;[1 1 1] Logout
  (bind _playerstate (`BlueprintAsyncActionGetPlayerState.AsyncGetPlayerState` ExitingController)
    (:`OnPlayerStateAcquired`
      ;;[1 1 1] We remove a player of the playerlist
      (`KismetArrayLibrary.Array_RemoveItem` (`self.PlayerStateList`) _playerstate))))

(event `self.K2_OnSetMatchState`
  (params (NewState :type Name))
  (switch `name` NewState
    (:`InProgress`
      (for _array_element (`self.PlayerStateList`)
        (message `TeamInterface.SetTeam` _array_element (`self.HuntedTeam`)))
      ;[1 1 1] The match start, a random player become infected
      (message `TeamInterface.SetTeam` (`KismetArrayLibrary.Array_Random` (`self.PlayerStateList`)) (`self.InfectedTeam`)))))

(fn `Get Player List`
  (returns (PlayerStateList :type "Array of PlayerState Object Reference") (DefaultTeam :type Integer))
  (return (`self.PlayerStateList`) (`self.DefaultTeam`)))

(fn `UserConstructionScript`
  (`parent.UserConstructionScript`))