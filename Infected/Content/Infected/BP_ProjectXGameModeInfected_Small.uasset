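; Game mode Blueprint, named as a small variant of the Infected mode, that keeps a list of connected players' player states.
; PostLogin and OnLogout each use an async node to wait for the controller's player state before adding it at the list's front or removing it.
; On logout it also prints the remaining players' names.
; It contains no infection or match logic, and BeginPlay and Tick are unused.
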(event `self.K2_PostLogin`
  (params (NewPlayer :type "PlayerController Object Reference"))
  ;[1 1 1] Login
  (bind _playerstate (`BlueprintAsyncActionGetPlayerState.AsyncGetPlayerState` NewPlayer)
    (:`OnPlayerStateAcquired`
      ;;[1 1 1] We add a new player to the player list
      (`KismetArrayLibrary.Array_Insert` (`self.PlayerStateList`) _playerstate))))

(event `self.K2_OnLogout`
  (params (ExitingController :type "Controller Object Reference"))
  (bind _playerstatelist (`self.PlayerStateList`))
  ;[1 1 1] Logout
  (bind _playerstate (`BlueprintAsyncActionGetPlayerState.AsyncGetPlayerState` ExitingController)
    (:`OnPlayerStateAcquired`
      ;;[1 1 1] We remove a player of the playerlist
      (`KismetArrayLibrary.Array_RemoveItem` _playerstatelist _playerstate)
      (for _array_element _playerstatelist
        (`KismetSystemLibrary.PrintString` (`PlayerState.GetPlayerName` _array_element))))))

(fn `UserConstructionScript`
  (`parent.UserConstructionScript`))