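; Juggernaut omnidirectional ground-pound melee weapon Blueprint, handling the cosmetic side of equip, charge, dive and landing.
; Equip and charge events drive local altitude and targeting widgets, attached audio, and a camera shake with dash effect on full charge.
; Fire spawns a danger hologram at the target for non-allies, plus launch sound and smoke trail on simulated proxies.
; Landing plays the explosion; landing, death, unequip and EndPlay wind down active effects.
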(event `Emit Warning`
  (`/Engine/EditorBlueprintResources/StandardMacros.Can Execute Cosmetic Events`
    (:`True`
      (bind _warning (`self.Warning`)
        (:`then`
          (`Actor.K2_DestroyActor` _warning))
        (:`else`
          _))
      (if (not (`ProjectXGameState.IsAlly` (`self.GetOwningCharacter`) (`GameplayStatics.GetPlayerController` 0)))
        (bind _returnvalue (`|SpawnActorFromClass` "/Game/Art/Effects/HologramMasterMaterials_V1/ExampleHolograms/Enervate_01/BP_Holograms_01_Danger.BP_Holograms_01_Danger_C" (`self.GetTargetTransform`) "Undefined" "OverrideRootScale" null null))
        (set `self.Warning` _returnvalue)))))

(event `self.ReceiveBeginPlay`
  (add `self.ChargeStartEvent` (delegate `ChargeStartEvent_Event_0`))
  (add `self.ChargeFinishedEvent` (delegate `ChargeFinishedEvent_Event_0`)))

(event `ChargeStartEvent_Event_0` :!signature `self.ChargeStartEvent`
  (params (TotalTime :type "Float (double-precision)") (TimeElapsed :type "Float (double-precision)"))
  (`|ExecutionSequence`
    (:`then_0`
      (`/Engine/EditorBlueprintResources/StandardMacros.IsValid` (`self.TargetingWidget`)
        (:`Is Valid`
          (`/Game/Blueprints/UI/Weapons/Groundpound/W_GroundPound.StartCharging` (`self.TargetingWidget`)))
        (:`Is Not Valid`
          (if (`Pawn.IsLocallyControlled` (`self.GetOwningCharacter`))
            (bind _returnvalue (`|CreateWidget` "/Game/Blueprints/UI/Weapons/Groundpound/W_GroundPound.W_GroundPound_C" (`self.GetOwningPlayerController`)))
            (bind _output_get (set `self.TargetingWidget` _returnvalue))
            (`UserWidget.AddToPlayerScreen` _output_get 0)
            (`/Game/Blueprints/UI/Weapons/Groundpound/W_GroundPound.StartCharging` (`self.TargetingWidget`))))))
    (:`then_1`
      (`/Engine/EditorBlueprintResources/StandardMacros.Can Execute Cosmetic Events`
        (:`True`
          (bind _returnvalue_2 (`GameplayStatics.SpawnSoundAttached` "/Game/Audio/Weapons/GroundPound/chargeup_Cue.chargeup_Cue" (`Actor.RootComponent` (`self.GetOwningCharacter`)) "None" (0.0 0.0 0.0) (struct) "KeepRelativeOffset" false 1.0 1.0 0.0 null null))
          (set `self.Sound` _returnvalue_2)
          (`HealthInterface.BindToDeathEvent` (`self.GetOwningCharacter`) (`|CreateDelegate` :!event `Died`)))))
    (:`then_2`
      (`/Engine/EditorBlueprintResources/StandardMacros.Can Execute Cosmetic Events`
        (:`True`
          (bind _returnvalue_3 (`GameplayStatics.SpawnSoundAttached` "/Game/Audio/Foley/jet_engine_startup_continuous_to_boost_power_Cue.jet_engine_startup_continuous_to_boost_power_Cue" (`Actor.RootComponent` (`self.GetOwningCharacter`)) "None" (0.0 0.0 0.0) (struct) "KeepRelativeOffset" false 1.0 1.0 0.0 null null))
          (bind _output_get_2 (set `self.JetSound` _returnvalue_3))
          (`AudioComponent.FadeIn` _output_get_2 1.0 1.0 0.0 "Linear"))))))

(event `ChargeFinishedEvent_Event_0` :!signature `self.ChargeFinishedEvent`
  (params (TotalTime :type "Float (double-precision)") (TimeElapsed :type "Float (double-precision)"))
  (bind _returnvalue (`self.GetOwningCharacter`))
  (if (!= TotalTime TimeElapsed)
    (`|ExecutionSequence`
      (:`then_0`
        (bind _jetsound (`self.JetSound`)
          (:`then`
            (`AudioComponent.FadeOut` _jetsound 0.5 0.0 "Linear"))
          (:`else`)))
      (:`then_1`
        (bind _sound (`self.Sound`)
          (:`then`
            (if (`AudioComponent.IsPlaying` _sound)
              (`AudioComponent.FadeOut` _sound 0.5 0.0 "Linear")))
          (:`else`)))
      (:`then_2`
        (bind _loopsound (`self.LoopSound`)
          (:`then`
            (`AudioComponent.FadeOut` _loopsound 0.5 0.0 "Linear"))
          (:`else`))))
    (else
      (`|ExecutionSequence`
        (:`then_0`
          (bind _altitudewidget (`self.AltitudeWidget`)
            (:`then`
              (`/Game/Blueprints/UI/Weapons/Groundpound/W_GroundPoundAltitude.Cleanup` (`self.AltitudeWidget`))
              (`/Game/Blueprints/UI/Weapons/Groundpound/W_GroundPoundAltitude.Cleanup` _altitudewidget))
            (:`else`)))
        (:`then_1`
          (if (`Pawn.IsLocallyControlled` _returnvalue)
            (`PlayerController.ClientStartCameraShake` :`self` (`ProjectXCharacter.GetPlayerController` _returnvalue) :`Shake` "/Game/ThirdPartyAssets/IBFPSStarterPack/Blueprints/BP_GroundPoundChargeShake.BP_GroundPoundChargeShake_C")
            (bind _asbp_project_xcharacter (cast `/Game/Blueprints/Gameplay/PlayerClasses/BP_ProjectXCharacter` (`self.GetOwningCharacter`)))
            (`/Game/Blueprints/Gameplay/PlayerClasses/BP_ProjectXCharacter.DashEffect` _asbp_project_xcharacter (struct :`R` 1.0 :`G` 0.017682 :`A` 1.0))))))))

(event `self.ReceiveEndPlay`
  (params (EndPlayReason :type "EEndPlayReason Enum" :default "Destroyed"))
  (`/Engine/EditorBlueprintResources/StandardMacros.IsValid` (`self.TargetingWidget`)
    (:`Is Valid`
      (`Widget.RemoveFromParent` (`self.TargetingWidget`)))
    (:`Is Not Valid`
      _))
  (`self.CleanEffectsUp`))

(event `self.K2_UnEquip`
  (`self.CleanEffectsUp`))

(event `self.K2_UnEquipComplete`
  (`self.CleanEffectsUp`))

(event `CleanEffectsUp`
  (`|ExecutionSequence`
    (:`then_0`
      (bind _loopsound (`self.LoopSound`)
        (:`then`
          (`AudioComponent.FadeOut` _loopsound 0.5 0.0 "Linear"))
        (:`else`)))
    (:`then_1`
      (bind _altitudewidget (`self.AltitudeWidget`)
        (:`then`
          (`/Game/Blueprints/UI/Weapons/Groundpound/W_GroundPoundAltitude.Cleanup` _altitudewidget))
        (:`else`)))
    (:`then_2`
      (bind _targetingwidget (`self.TargetingWidget`)
        (:`then`
          (`/Game/Blueprints/UI/Weapons/Groundpound/W_GroundPound.ConcludeEffects` _targetingwidget false))
        (:`else`)))
    (:`then_3`
      (`KismetSystemLibrary.Delay` 0.5)
      (bind _loopsound_2 (`self.LoopSound`)
        (:`then`
          (`AudioComponent.Stop` _loopsound_2))
        (:`else`)))
    (:`then_4`
      (bind _jetsound (`self.JetSound`)
        (:`then`
          (`AudioComponent.FadeOut` _jetsound 0.5 0.0 "Linear"))
        (:`else`)))
    (:`then_5`
      (bind _sound (`self.Sound`)
        (:`then`
          (`AudioComponent.FadeOut` _sound 0.5 0.0 "Linear"))
        (:`else`)))
    (:`then_6`
      (bind _divesmokeparticle (`self.DiveSmokeParticle`)
        (:`then`
          (`self.Deactivate` _divesmokeparticle))
        (:`else`)))
    (:`then_7`
      (bind _warning (`self.Warning`)
        (:`then`
          (`/Game/Art/Effects/HologramMasterMaterials_V1/ExampleHolograms/Enervate_01/BP_Holograms_01_Danger.Cleanup` _warning))
        (:`else`)))))

(event `self.OnLandedGround`
  (params (Hit :type "HitResult Structure (by ref)"))
  (bind _returnvalue (`Actor.K2_GetActorLocation` (`self.GetOwningCharacter`)))
  (`|ExecutionSequence`
    (:`then_0`
      (bind _jetsound (`self.JetSound`)
        (:`then`
          (`AudioComponent.FadeOut` _jetsound 0.5 0.0 "Linear"))
        (:`else`)))
    (:`then_1`
      (`GameplayStatics.PlaySoundAtLocation` "/Game/Audio/Explosions/Explosion_Large_Cue.Explosion_Large_Cue" _returnvalue (struct) 1.0 1.0 0.0 null null null)
      (`GameplayStatics.SpawnEmitterAtLocation` "/Game/Art/Effects/Particles/Explosions/P_Explosion_GroundPound.P_Explosion_GroundPound" _returnvalue)
      (`|ExecutionSequence`
        (:`then_0`
          (bind _loopsound (`self.LoopSound`)
            (:`then`
              (if (`AudioComponent.IsPlaying` _loopsound)
                (`AudioComponent.FadeOut` _loopsound 0.5 0.0 "Linear")))
            (:`else`)))
        (:`then_1`
          (bind _warning (`self.Warning`)
            (:`then`
              (`/Game/Art/Effects/HologramMasterMaterials_V1/ExampleHolograms/Enervate_01/BP_Holograms_01_Danger.Cleanup` _warning))
            (:`else`)))))
    (:`then_2`
      (bind _divesmokeparticle (`self.DiveSmokeParticle`)
        (:`then`
          (`self.Deactivate` _divesmokeparticle))
        (:`else`)))))

(event `self.K2_Equip`
  (`/Engine/EditorBlueprintResources/StandardMacros.Can Execute Cosmetic Events`
    (:`True`
      (bind _returnvalue (`GameplayStatics.SpawnSoundAttached` "/Game/Audio/Weapons/GroundPound/activate_CUE.activate_CUE" (`Actor.RootComponent` (`self.GetOwningCharacter`)) "None" (0.0 0.0 0.0) (struct) "KeepRelativeOffset" false 1.0 1.0 0.0 null null))
      (set `self.LoopSound` _returnvalue)
      (if (`Pawn.IsLocallyControlled` (`self.GetOwningCharacter`))
        (bind _returnvalue_2 (`|CreateWidget` "/Game/Blueprints/UI/Weapons/Groundpound/W_GroundPoundAltitude.W_GroundPoundAltitude_C" (`self.GetOwningPlayerController`)))
        (`/Game/Blueprints/UI/Weapons/Groundpound/W_GroundPoundAltitude.TogglePowerBar` _returnvalue_2 false)
        (bind _output_get (set `self.AltitudeWidget` _returnvalue_2))
        (`UserWidget.AddToViewport` _output_get 0)))))

(event `Died`
  (params (Victim :type "Actor Object Reference") (Damage :type "Float (double-precision)") (DamageEvent :type "DamageEvent Structure (by ref)") (EventInstigator :type "Controller Object Reference") (DamageCauser :type "Actor Object Reference") (InstigatorPlayerState :type "PlayerState Object Reference"))
  (`|ExecutionSequence`
    (:`then_0`
      (bind _jetsound (`self.JetSound`)
        (:`then`
          (if (`AudioComponent.IsPlaying` _jetsound)
            (`AudioComponent.FadeOut` _jetsound 0.5 0.0 "Linear")))
        (:`else`)))
    (:`then_1`
      (bind _divesmokeparticle (`self.DiveSmokeParticle`)
        (:`then`
          (`self.Deactivate` _divesmokeparticle))
        (:`else`)))))

(event `self.K2_Fire`
  (params (Mode :type Byte))
  (bind _returnvalue (`self.GetOwner`))
  (`parent.K2_Fire` Mode)
  (`|ExecutionSequence`
    (:`then_0`
      (`self.Emit Warning`))
    (:`then_1`
      (`/Engine/EditorBlueprintResources/StandardMacros.IsValid` _returnvalue
        (:`Is Valid`
          (if (`|EnumEquality` (`Actor.GetLocalRole` _returnvalue) "ROLE_SimulatedProxy")
            (`GameplayStatics.SpawnSoundAtLocation` "/Game/Audio/Abilities/Groundpound/GroundPound_Launch_Cue.GroundPound_Launch_Cue" (`Actor.K2_GetActorLocation` _returnvalue) (struct) 0.8 1.0 0.0 null null)
            (bind _divesmokeparticle (`self.DiveSmokeParticle`)
              (:`then`
                (if (not (`self.IsActive` _divesmokeparticle))
                  (`self.Activate` _divesmokeparticle true)))
              (:`else`
                (bind _returnvalue_2 (`GameplayStatics.SpawnEmitterAttached` "/Game/Art/Effects/Particles/Trails/PlayerTrails/P_PlayerTrail_Smoke.P_PlayerTrail_Smoke" (`Actor.RootComponent` _returnvalue) "None" (0.0 0.0 0.0) (struct) (1.0 1.0 1.0) "SnapToTarget" false))
                (set `self.DiveSmokeParticle` _returnvalue_2)))))))))

(event `self.K2_ToggleDesignatorMarker`
  (params (NewDesignatorMarker :type "Actor Object Reference"))
  (`/Engine/EditorBlueprintResources/StandardMacros.IsValid` NewDesignatorMarker
    (:`Is Valid`
      (set `self.Designator Marker` NewDesignatorMarker))))