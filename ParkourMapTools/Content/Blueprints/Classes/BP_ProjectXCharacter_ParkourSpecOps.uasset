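; Parkour SpecOps character Blueprint that adds respawning to the start point or the latest checkpoint.
; BeginPlay stores the spawn location as both start and initial checkpoint; no graph here updates the checkpoint afterwards.
; Both teleports share TeleportToPosition, which sets the transform from a location and zeroes movement velocity on success.
; Returning to start also increments a restart counter, even if the move fails.
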(event `self.ReceiveBeginPlay`
  (`parent.ReceiveBeginPlay`)
  (bind _output_get (set `self.DefaultSpawnLocation` (`self.K2_GetActorLocation` self)))
  (set `self.CheckpointLocation` _output_get))

(fn `ResetVelocity`
  (set `MovementComponent.Velocity` (0.0 0.0 0.0) (`self.GetMovementComponent` self)))

(fn `TeleportToCheckpoint`
  (returns (HasTP :type Boolean))
  (bind _hastp (`self.TeleportToPosition` (`KismetMathLibrary.Conv_VectorToTransform` (`self.CheckpointLocation`))))
  (return _hastp))

(fn `TeleportToPosition`
  (params (TeleportPosition :type "Transform Structure (by ref)"))
  (returns (HasTP :type Boolean))
  (bind (_sweephitresult _returnvalue) (`self.K2_SetActorTransform` TeleportPosition))
  (if _returnvalue
    (`self.ResetVelocity`)
    (return _returnvalue)))

(fn `TeleportToStart`
  (returns (HasTP :type Boolean))
  (bind _hastp (`self.TeleportToPosition` (`KismetMathLibrary.Conv_VectorToTransform` (`self.DefaultSpawnLocation`))))
  (`/Engine/EditorBlueprintResources/StandardMacros.IncrementInt` (`self.RestartAmount`)
    (:`  `
      (return _hastp))))

(fn `UserConstructionScript`
  (`parent.UserConstructionScript`))