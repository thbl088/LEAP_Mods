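; Ducky personal vehicle, a child Blueprint that layers cosmetic boosters, rolls and team colours onto its parent.
; BeginPlay sockets the boosters to the mesh and caches the MechMoose AnimInstance, which receives boost state.
; Smoothed forward acceleration, adjusted for boosting and grounding, scales rear afterburner size and distortion.
; MeshPivotPoint spins during airborne boosts and eases upright otherwise, while BoostEffects plays a locked, eased barrel roll directed by sideways velocity.
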(event `self.ReceiveBeginPlay`
  (`/Engine/EditorBlueprintResources/StandardMacros.Can Execute Cosmetic Events`
    (:`True`
      (`|ExecutionSequence`
        (:`then_0`
          (`KismetArrayLibrary.Array_Clear` (`self.BottomBoosters`))
          (set `self.BottomBoosters` (`|MakeArray` (`self.BottomBooster`))))
        (:`then_1`
          (`KismetArrayLibrary.Array_Clear` (`self.RearBoosters`))
          (set `self.RearBoosters` (`|MakeArray` (`self.PSN_Afterburners_Controllable1`) (`self.PSN_Afterburners_Controllable2`) (`self.AfterBurner1`) (`self.AfterBurner2`)))
          (`FXSystemComponent.SetFloatParameter` (`self.PSN_Afterburners_Controllable1`) "User.DistortionScaleY" 0.0)
          (`FXSystemComponent.SetFloatParameter` (`self.PSN_Afterburners_Controllable2`) "User.DistortionScaleY" 0.0)
          (`FXSystemComponent.SetFloatParameter` (`self.AfterBurner2`) "User.DistortionScaleY" 0.0)
          (`FXSystemComponent.SetFloatParameter` (`self.AfterBurner1`) "User.DistortionScaleY" 0.0))
        (:`then_2`
          (`SceneComponent.K2_AttachToComponent` (`self.AfterBurner1`) (`self.Mesh`) "Afterburner1" "SnapToTarget" "SnapToTarget" "SnapToTarget" true)
          (`SceneComponent.K2_AttachToComponent` (`self.PSN_Afterburners_Controllable1`) (`self.Mesh`) "Afterburner1" "SnapToTarget" "SnapToTarget" "SnapToTarget" true))
        (:`then_3`
          (`SceneComponent.K2_AttachToComponent` (`self.AfterBurner2`) (`self.Mesh`) "Afterburner2" "SnapToTarget" "SnapToTarget" "SnapToTarget" true)
          (`SceneComponent.K2_AttachToComponent` (`self.PSN_Afterburners_Controllable2`) (`self.Mesh`) "Afterburner2" "SnapToTarget" "SnapToTarget" "SnapToTarget" true))
        (:`then_4`
          (`SceneComponent.K2_AttachToComponent` (`self.BottomBooster`) (`self.Mesh`) "BottomBooster" "SnapToTarget" "SnapToTarget" "SnapToTarget" true))
        (:`then_5`
          (`parent.ReceiveBeginPlay` :!label _label)
          (`/Engine/EditorBlueprintResources/StandardMacros.Can Execute Cosmetic Events`
            (:`True`
              (bind _asabp_personal_vehicle_mech_moose (cast `/Game/Art/Vehicles/Animations/MechMoose/ABP_PersonalVehicle_MechMoose` (`SkeletalMeshComponent.GetAnimInstance` (`self.Mesh`))))
              (set `self.AnimInstance` _asabp_personal_vehicle_mech_moose))))))
    (:`False`
      (goto _label))))

(event `self.OnBoostingStarted`
  (`parent.OnBoostingStarted`)
  (bind _animinstance (`self.AnimInstance`)
    (:`then`
      (`/Game/Art/Vehicles/Animations/MechMoose/ABP_PersonalVehicle_MechMoose.Boost` _animinstance))
    (:`else`)))

(event `self.OnBoostingStopped`
  (`parent.OnBoostingStopped`)
  (bind _animinstance (`self.AnimInstance`)
    (:`then`
      (`/Game/Art/Vehicles/Animations/MechMoose/ABP_PersonalVehicle_MechMoose.StopBoost` _animinstance))
    (:`else`)))

(event `self.Set Valid Team Colour`
  (bind _returnvalue (`KismetMathLibrary.Conv_LinearColorToVector` (`ProjectXGameState.GetTargetColour` self "None" (`GameplayStatics.GetPlayerController` 0))))
  (`parent.Set Valid Team Colour`)
  (`MeshComponent.SetVectorParameterValueOnMaterials` (`self.Mesh`) "TeamColour1" _returnvalue)
  (`MeshComponent.SetVectorParameterValueOnMaterials` (`self.Mesh`) "EmissiveColour" (* _returnvalue 10.0)))

(event `self.ReceiveTick`
  (params (DeltaSeconds :type "Float (single-precision)"))
  (bind (_relativerotation_roll _relativerotation_pitch _relativerotation_yaw) (`KismetMathLibrary.BreakRotator` (`SceneComponent.RelativeRotation` (`self.MeshPivotPoint`))))
  (`parent.ReceiveTick` DeltaSeconds)
  (`/Engine/EditorBlueprintResources/StandardMacros.Can Execute Cosmetic Events`
    (:`True`
      (set `self.Time` (+ (`self.Time`) (* (* DeltaSeconds (`KismetMathLibrary.SelectFloat` -1.0 1.0 (`self.IsMovingForward`))) (`KismetMathLibrary.Lerp` 0.0 3.0 (`KismetMathLibrary.FClamp` (/ (`KismetMathLibrary.VSize` (`self.GetVelocity`)) (* (`CharacterMovementComponent.MaxWalkSpeed` (`self.CharacterMovement`)) (`self.GetBoostMultiplier`))))))))
      (`self.AnimInstance`
        (:`then`
          (if (and (not (`ProjectXVehicleMovementComponent.IsGroundedInFlyingMode` (cast `ProjectXVehicleMovementComponent` (`self.CharacterMovement`) :!pure true))) (`self.IsBoosting`))
            (`SceneComponent.K2_AddRelativeRotation` (`self.MeshPivotPoint`) (`KismetMathLibrary.MakeRotator` (* (`self.DeltaTime`) 250.0)) false false)
            (else
              (`SceneComponent.K2_SetRelativeRotation` (`self.MeshPivotPoint`) (`KismetMathLibrary.MakeRotator` (`KismetMathLibrary.Lerp` _relativerotation_roll 0.0 (* (`self.DeltaTime`) 2.0)) _relativerotation_pitch _relativerotation_yaw) false false))))
        (:`else`)))))

(event `self.BoostEffects`
  (if (not (`self.bDoingCosmeticJump`))
    (`/Engine/EditorBlueprintResources/StandardMacros.DoOnce` false :!label _label_2
      (:`Completed`
        (`parent.BoostEffects`)
        (`/Engine/EditorBlueprintResources/StandardMacros.Can Execute Cosmetic Events`
          (:`True`
            (`|ExecutionSequence`
              (:`then_0`
                (`Interpolator.ClearInterpolation` self (`self.SpinInterp`))
                (`Interpolator.ClearInterpolation` self)
                (bind _returnvalue (`Interpolator.InterpolateOverTime` 0.0 3.0 0.0 (`KismetMathLibrary.SelectFloat` 1080.0 -1080.0 (> (`KismetMathLibrary.Dot_VectorVector` (`KismetMathLibrary.Normal` (`self.GetVelocity`)) (`self.GetActorRightVector`)) 0.0)) "EaseOut" (delegate `BarrelRoll`) (delegate `Stop Roll`)))
                (set `self.BoostSpinInterp` _returnvalue))
              (:`then_1`
                (bind _animinstance (`self.AnimInstance`)
                  (:`then`
                    (`/Game/Art/Vehicles/Animations/MechMoose/ABP_PersonalVehicle_MechMoose.Toggle CosmeticBoosting` _animinstance true))
                  (:`else`))))))))))

(event `ResetRotation`
  (`self.ResetBoostLock`)
  (goto _label_2 :!via `Reset`))

(event `BarrelRoll`
  (params (Value :type "Float (double-precision)"))
  (bind (_relativerotation_roll _relativerotation_pitch _relativerotation_yaw) (`KismetMathLibrary.BreakRotator` (`SceneComponent.RelativeRotation` (`self.MeshPivotPoint`))))
  (`SceneComponent.K2_SetRelativeRotation` (`self.MeshPivotPoint`) (`KismetMathLibrary.MakeRotator` Value _relativerotation_pitch _relativerotation_yaw) false false))

(event `Stop Roll`
  (params (Value :type "Float (double-precision)"))
  (bind _animinstance (`self.AnimInstance`)
    (:`then`
      (`/Game/Art/Vehicles/Animations/MechMoose/ABP_PersonalVehicle_MechMoose.Toggle CosmeticBoosting` _animinstance false)
      (`self.ResetRotation`))
    (:`else`)))

(event `self.Handle Cosmetic Boosters`
  (params (Delta :type "Float (single-precision)"))
  (bind _returnvalue (`self.IsBoosting`))
  (bind _returnvalue_2 (`KismetMathLibrary.Lerp` (`self.BoosterMinSize`) (`self.BoosterMaxSize`) (`self.LerpedAcceleration`)))
  (bind _returnvalue_3 (`KismetMathLibrary.VSize` (/ (* (`self.GetVehicleRelativeAcceleration`) (1.0 0.0 0.0)) (`CharacterMovementComponent.GetMaxAcceleration` (`self.CharacterMovement`)))))
  (bind _returnvalue_4 (* _returnvalue_3 (`self.BoostingBoostSizeMultiplier`)))
  (`/Engine/EditorBlueprintResources/StandardMacros.Can Execute Cosmetic Events`
    (:`True`
      (bind _asproject_xvehicle_movement_component (cast `ProjectXVehicleMovementComponent` (`self.CharacterMovement`)))
      (`|ExecutionSequence`
        (:`then_0`
          (set `self.LerpedAcceleration` (`KismetMathLibrary.FInterpTo` (`self.LerpedAcceleration`) (`KismetMathLibrary.SelectFloat` (`KismetMathLibrary.SelectFloat` (* _returnvalue_4 0.5) 0.0 _returnvalue) (`KismetMathLibrary.SelectFloat` _returnvalue_4 _returnvalue_3 _returnvalue) (`ProjectXVehicleMovementComponent.IsGroundedInFlyingMode` _asproject_xvehicle_movement_component)) Delta 5.0)))
        (:`then_1`
          (for _array_element (`self.RearBoosters`)
            (`/Engine/EditorBlueprintResources/StandardMacros.IsValid` _array_element
              (:`Is Valid`
                (`NiagaraComponent.SetVariableVec2` _array_element "User.BurnerScale" (`KismetMathLibrary.MakeVector2D` 1.0 _returnvalue_2))
                (`NiagaraComponent.SetVariableFloat` _array_element "User.DistortionScaleY" _returnvalue_2)))))))))

(fn `UserConstructionScript`
  (`parent.UserConstructionScript`))